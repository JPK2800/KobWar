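; Spectator pawn that lets a player look around while in spectating mode and back out of it.
; SetSpectatingMode toggles control, adding or removing the spectating widget and switching mouse cursor and input mode.
; Turn and look axes rotate the view only while in control.
; A menu-back event, bound through BP_PlayerController on BeginPlay, cancels spectating via its BPCTeamClassControl component and turns the mode off.
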(event `self.ReceiveBeginPlay`
  (bind _asbp_player_controller (cast `/Game/KobWar/Controllers/BP_PlayerController` (`GameplayStatics.GetPlayerController` 0)))
  (add `GamePlayerController.OnMenuBack` _asbp_player_controller (`|CreateDelegate` :!event `MenuBack`)))

(event `InputAxis|TurnRate`
  (params (AxisValue :type "Float (single-precision)"))
  (if (`self.InControl`)
    (`self.AddControllerYawInput` AxisValue)))

(event `InputAxis|Turn`
  (params (AxisValue :type "Float (single-precision)"))
  (if (`self.InControl`)
    (`self.AddControllerYawInput` AxisValue)))

(event `InputAxis|LookUpRate`
  (params (AxisValue :type "Float (single-precision)"))
  (if (`self.InControl`)
    (`self.AddControllerPitchInput` AxisValue)))

(event `InputAxis|LookUp`
  (params (AxisValue :type "Float (single-precision)"))
  (if (`self.InControl`)
    (`self.AddControllerPitchInput` AxisValue)))

(event `MenuBack`
  (params (Press :type Boolean) (Release :type Boolean))
  (if Press
    (if (`self.InControl`)
      (bind _asbp_player_controller (cast `/Game/KobWar/Controllers/BP_PlayerController` (`self.GetController`)))
      (`/Game/KobWar/LogicComponents/ControllerTeamClassControl/BPC_TeamClassControl.CancelSpectating` (`/Game/KobWar/Controllers/BP_PlayerController.BPC_TeamClassControl` _asbp_player_controller))
      (`self.SetSpectatingMode` false))))

(fn `SetSpectatingMode`
  (params (Toggle :type Boolean))
  (bind _returnvalue (`GameplayStatics.GetPlayerController` 0))
  (bind _spectatingwidget (`self.SpectatingWidget`))
  (bind _output_get (set `self.InControl` Toggle))
  (if _output_get
    (bind _returnvalue_2 (`|CreateWidget` "/Game/KobWar/Spectating/WBP_SpectatingWidget.WBP_SpectatingWidget_C" _returnvalue))
    (`UserWidget.AddToPlayerScreen` _returnvalue_2 0)
    (set `self.SpectatingWidget` _returnvalue_2)
    (set `PlayerController.bShowMouseCursor` false _returnvalue)
    (`WidgetBlueprintLibrary.SetInputMode_GameOnly` _returnvalue)
    (else
      (`/Engine/EditorBlueprintResources/StandardMacros.IsValid` _spectatingwidget
        (:`Is Valid`
          (`Widget.RemoveFromParent` _spectatingwidget)
          (set `self.SpectatingWidget` null)
          (set `PlayerController.bShowMouseCursor` true _returnvalue)
          (`WidgetBlueprintLibrary.SetInputMode_GameAndUIEx` _returnvalue null))))))

(fn `UserConstructionScript`)