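; KobWar player controller that handles team and class selection, pawn spawning and menu input pausing.
; BPC_TeamClassControl events trigger an immediate spawn before game start, queue a respawn afterwards, or switch to spectating.
; Server-prefixed events spawn and possess character, spectator or preview pawns and relay team requests to the game mode, answering through Owner-prefixed events.
; It also shows pregame and respawn timers, plus a debug-key binding menu.
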(event `self.ReceiveBeginPlay`
  (`KismetSystemLibrary.K2_SetTimerDelegate` (delegate `OnInitWait`) 0.1))

(event `OnInitWait`
  (if (`self.IsLocalPlayerController`)
    (`self.SpawnPregameTimerWidget`)))

(event `self.BPC_TeamClassControl.ClassEquipmentSet`
  (params (ClassName :type Name) (ClassEquipment :type Name) (Skeleton :type Name))
  (set `self.ClassName` ClassName)
  (set `self.ClassEquipment` ClassEquipment)
  (set `self.Skeleton` Skeleton)
  (bind _asbp_game_state (cast `/Game/KobWar/GameModeLogic/BP_GameState` (`GameplayStatics.GetGameState`)))
  (if (`/Game/KobWar/GameModeLogic/BP_GameState.GameStarted` _asbp_game_state)
    (`self.ServerAddToRespawnQueue` self)
    (else
      (`self.OwnerTriggerSpawn`))))

(event `self.BPC_TeamClassControl.SpectatorTeamSet`
  (bind _returnvalue (`self.K2_GetPawn`))
  (`/Engine/EditorBlueprintResources/StandardMacros.IsValid` _returnvalue
    (:`Is Valid`
      (bind _asbp_inaction_spectator_pawn (cast `/Game/KobWar/BP_InactionSpectatorPawn` _returnvalue)
        (:`then`
          (`/Game/KobWar/BP_InactionSpectatorPawn.SetSpectatingMode` _asbp_inaction_spectator_pawn true))
        (:`CastFailed`
          (`self.ServerDespawnActor`)
          (`self.ServerSpawnSpectatorActor` :!label _label))))
    (:`Is Not Valid`
      (goto _label))))

(event `Key|AnyKey` :consume false :overrideparent false
  (params (Key :type "Key Structure"))
  (:`Pressed`
    (`/Game/KobWar/LogicComponents/Input/BPC_InputDataComponent.AnyKeyPressed` (`self.BPC_InputDataComponent`) Key)))

(event `Key|I`
  (params (Key :type "Key Structure"))
  ;[1 1 1] Debug
  (:`Pressed`
    (`self.SpawnKeyBindingWidget`)))

(event `ServerSpawnActor`
  (params (CharClass :type "/Game/KobWar/BP_PlayerCharacterBase Class Reference") (Team :type Byte) (ClassName :type Name) (EquipmentName :type Name))
  (bind _returnvalue (`|SpawnActorFromClass` CharClass (`KismetMathLibrary.MakeTransform` (500.0 500.0 500.0)) "Undefined" "OverrideRootScale" self ClassName EquipmentName Team null))
  (`self.Possess` _returnvalue)
  (`self.OwnerUpdateMenuOpenOnSpawn` _returnvalue))

(event `ServerDespawnActor`
  (bind _returnvalue (`self.K2_GetPawn`))
  (`/Engine/EditorBlueprintResources/StandardMacros.IsValid` _returnvalue
    (:`Is Valid`
      (`self.K2_DestroyActor` _returnvalue))))

(event `ServerSpawnSpectatorActor`
  (bind _returnvalue (`|SpawnActorFromClass` "/Game/KobWar/BP_InactionSpectatorPawn.BP_InactionSpectatorPawn_C" (`KismetMathLibrary.MakeTransform` (500.0 500.0 500.0)) "Undefined" "OverrideRootScale" self false null))
  (`self.Possess` _returnvalue))

(event `ServerSpawnCharPreviewActor`
  (bind _returnvalue (`|SpawnActorFromClass` "/Game/KobWar/GameModeLogic/ClassPreviewPawn/BP_ClassPreviewPawn.BP_ClassPreviewPawn_C" (`KismetMathLibrary.MakeTransform` (`KismetMathLibrary.MakeVector` (`KismetMathLibrary.Conv_IntToDouble` (* (`GameplayStatics.GetPlayerControllerID` self) 5000)) 0.0 -5000.0)) "Undefined" "OverrideRootScale" self null))
  (`self.Possess` _returnvalue))

(event `ServerRequestSetTeamId`
  (params (TeamId :type Byte) (PlayerController :type "/Game/KobWar/Controllers/BP_PlayerController Object Reference"))
  (bind _askob_war_game_mode (cast `KobWarGameMode` (`GameplayStatics.GetGameMode`)))
  (bind _returnvalue (`KobWarGameMode.SetPlayerTeam` _askob_war_game_mode PlayerController TeamId false))
  (if _returnvalue
    (`self.OwnerSetTeamUpdate` TeamId)))

(event `ServerAddToRespawnQueue`
  (params (PlayerController :type "/Game/KobWar/Controllers/BP_PlayerController Object Reference"))
  (bind _askob_war_game_mode (cast `KobWarGameMode` (`GameplayStatics.GetGameMode`)))
  (bind _returnvalue (`KobWarGameMode.AddToRespawnQueue` _askob_war_game_mode PlayerController))
  (if _returnvalue
    (`self.OwnerSpawnRespawnTimer`)))

(event `OwnerSetTeamUpdate`
  (params (TeamId :type Byte))
  (`/Game/KobWar/LogicComponents/ControllerTeamClassControl/BPC_TeamClassControl.UpdateTeamSelected` (`self.BPC_TeamClassControl`) TeamId))

(event `OwnerTriggerSpawn`
  (bind _classname (`self.ClassName`))
  (bind _classequipment (`self.ClassEquipment`))
  (bind (_charclass _found) (`/Game/KobWar/Controllers/SpawnData/BPFL_GetSkeletonClass.GetSpawnActor` (`self.Skeleton`) _classname _classequipment))
  (if _found
    (`self.ServerSpawnActor` _charclass (`/Game/KobWar/LogicComponents/ControllerTeamClassControl/BPC_TeamClassControl.TeamSelected` (`self.BPC_TeamClassControl`)) _classname _classequipment)))

(event `OwnerSpawnRespawnTimer`
  (bind _asbp_game_state (cast `/Game/KobWar/GameModeLogic/BP_GameState` (`GameplayStatics.GetGameState`)))
  (bind _time (`/Game/KobWar/GameModeLogic/BP_GameState.GetTimeUntilRespawn` _asbp_game_state))
  (bind _returnvalue (`|CreateWidget` "/Game/KobWar/PregameTimerWidget/WBP_RespawnTimerWidget.WBP_RespawnTimerWidget_C" self (+ (`KismetMathLibrary.Now`) (`KismetMathLibrary.MakeTimespan` 0 0 0 (`KismetMathLibrary.FTrunc` _time)))))
  (`UserWidget.AddToPlayerScreen` _returnvalue 0))

(event `OwnerUpdateMenuOpenOnSpawn`
  (params (PlayerCharacter :type "/Game/KobWar/BP_PlayerCharacterBase Object Reference"))
  (`KobWarCharacter.SetPausedInputsForMenu` PlayerCharacter (`self.IsMenuOpen`)))

(event `ServerChangePlayerTeam`
  (params (NewTeam :type Byte))
  (`|ExecutionSequence`
    (:`then_0`
      (bind _askob_war_game_mode (cast `KobWarGameMode` (`GameplayStatics.GetGameMode`)))
      (`KobWarGameMode.SetPlayerTeam` _askob_war_game_mode null NewTeam true))))

(fn `PauseCharacterInputsForMenu`
  (bind _returnvalue (`GameplayStatics.GetPlayerPawn` 0))
  (set `self.IsMenuOpen` true)
  (`|ExecutionSequence`
    (:`then_0`
      (bind _asbp_inaction_spectator_pawn (cast `/Game/KobWar/BP_InactionSpectatorPawn` _returnvalue)
        (:`then`
          (set `/Game/KobWar/BP_InactionSpectatorPawn.InControl` false _asbp_inaction_spectator_pawn))
        (:`CastFailed`
          (bind _asbp_player_character_base (cast `/Game/KobWar/BP_PlayerCharacterBase` _returnvalue))
          (`KobWarCharacter.SetPausedInputsForMenu` _asbp_player_character_base true))))))

(fn `SpawnKeyBindingWidget`
  (bind _returnvalue (`|CreateWidget` "/Game/KobWar/Inputs/WBP_InputWidget.WBP_InputWidget_C" self))
  (bind (_inputmap _orderednames) (`/Game/KobWar/LogicComponents/Input/BPC_InputDataComponent.LoadMappingsButtons` (`self.BPC_InputDataComponent`)))
  (`/Game/KobWar/Inputs/WBP_InputWidget.LoadCurrentSettings` _returnvalue _inputmap _orderednames)
  (`UserWidget.AddToPlayerScreen` _returnvalue 0)
  (set `self.IsMenuOpen` true)
  (`self.PauseCharacterInputsForMenu`))

(fn `SpawnPregameTimerWidget`
  (bind _asbp_game_state (cast `/Game/KobWar/GameModeLogic/BP_GameState` (`GameplayStatics.GetGameState`)))
  (if (not (`/Game/KobWar/GameModeLogic/BP_GameState.GameStarted` _asbp_game_state))
    (bind _returnvalue (`|CreateWidget` "/Game/KobWar/PregameTimerWidget/WBP_PregameTimerWidget.WBP_PregameTimerWidget_C" self (`/Game/KobWar/GameModeLogic/BP_GameState.TimeToTriggerGame` _asbp_game_state)))
    (`UserWidget.AddToPlayerScreen` _returnvalue 0)))

(fn `UnpauseCharacterInputsForMenu`
  (bind _returnvalue (`GameplayStatics.GetPlayerPawn` 0))
  (set `self.IsMenuOpen` false)
  (`|ExecutionSequence`
    (:`then_0`
      (bind _asbp_inaction_spectator_pawn (cast `/Game/KobWar/BP_InactionSpectatorPawn` _returnvalue)
        (:`then`
          (set `/Game/KobWar/BP_InactionSpectatorPawn.InControl` true _asbp_inaction_spectator_pawn))
        (:`CastFailed`
          (bind _asbp_player_character_base (cast `/Game/KobWar/BP_PlayerCharacterBase` _returnvalue))
          (`KobWarCharacter.SetPausedInputsForMenu` _asbp_player_character_base false))))))

(fn `UserConstructionScript`)