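; Kobold Assassin character variant that fights with daggers, built on a parent character Blueprint.
; On BeginPlay and again on possession, it passes its action component and team ID to LoadKoboldDaggersData.
; The returned main-hand and off-hand classes feed the equipment handler component, and the animation index updates the animations.
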(event `self.ReceiveBeginPlay`
  (bind _bpc_equipmenthandler (`self.BPC_EquipmentHandler`))
  (`parent.ReceiveBeginPlay`)
  (bind (_lightattackdata _heavyattackdata _dodgedata _staggerdata _stagger2data _landdata _weaponskilldata _runningattackdata _backstepdata _specialaction1 _specialaction2 _mainhandclass _offhandclass _animationindex) (`/Game/KobWar/Equipment/BPFL_LoadEquipAnimData.LoadKoboldDaggersData` (`self.ActionControl`) 0 0 0 (`self.GenericTeamId`)))
  (`/Game/KobWar/LogicComponents/Equipment/BPC_EquipmentHandler.UpdateMainEquipData` _bpc_equipmenthandler _mainhandclass)
  (`/Game/KobWar/LogicComponents/Equipment/BPC_EquipmentHandler.UpdateOffhandEquipData` _bpc_equipmenthandler _offhandclass)
  (`self.UpdateAnimations` _animationindex))

(event `self.ReceivePossessed`
  (params (NewController :type "Controller Object Reference"))
  (bind _bpc_equipmenthandler (`self.BPC_EquipmentHandler`))
  (bind (_lightattackdata _heavyattackdata _dodgedata _staggerdata _stagger2data _landdata _weaponskilldata _runningattackdata _backstepdata _specialaction1 _specialaction2 _mainhandclass _offhandclass _animationindex) (`/Game/KobWar/Equipment/BPFL_LoadEquipAnimData.LoadKoboldDaggersData` (`self.ActionControl`) 0 0 0 (`self.GenericTeamId`)))
  (`/Game/KobWar/LogicComponents/Equipment/BPC_EquipmentHandler.UpdateMainEquipData` _bpc_equipmenthandler _mainhandclass)
  (`/Game/KobWar/LogicComponents/Equipment/BPC_EquipmentHandler.UpdateOffhandEquipData` _bpc_equipmenthandler _offhandclass)
  (`self.UpdateAnimations` _animationindex))

(fn `UserConstructionScript`
  (`parent.UserConstructionScript`))