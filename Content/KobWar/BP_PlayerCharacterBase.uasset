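; Base player character for KobWar that handles networked animation, aiming and team-based class cosmetics loaded at begin play.
; Action animations and lock-on state play locally, then relay through server and multicast to an interface-driven anim instance.
; Aiming state and control rotation go to the server, with an OnRep switching animation and controller-yaw facing.
; Each tick, the local player interpolates boom length, offset and FOV into an over-the-shoulder aim view.
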(event `self.ReceiveBeginPlay`
  (`self.Initialization`))

(event `self.ReceiveTick`
  (params (DeltaSeconds :type "Float (single-precision)"))
  (`self.UpdateAimRotStep` DeltaSeconds)
  (`self.InterpAimCamStep` DeltaSeconds))

(event `LocalPlayActionAnimation`
  (params (Animation :type "AnimMontage Object Reference"))
  (`/Engine/EditorBlueprintResources/StandardMacros.IsValid` Animation
    (:`Is Valid`
      (`/Engine/EditorBlueprintResources/StandardMacros.IsValid` Animation
        (:`Is Valid`
          (message `/Game/KobWar/CharacterAssets/Kobold/BPI_AnimationChar.SetSinglePlayAnimation` (`self.AnimInstance`) Animation)
          (if (`self.IsLocallyControlled`)
            (`self.ServerPlayActionAnimation` Animation)))))))

(event `ServerPlayActionAnimation`
  (params (Animation :type "AnimMontage Object Reference"))
  (`self.MulticastPlayActionAnimation` Animation))

(event `MulticastPlayActionAnimation`
  (params (Animation :type "AnimMontage Object Reference"))
  (if (not (`self.IsLocallyControlled`))
    (`self.LocalPlayActionAnimation` Animation)))

(event `self.PlayActionAnimation`
  (params (Animation :type "AnimMontage Object Reference"))
  (`self.LocalPlayActionAnimation` Animation))

(event `self.BPC_LockOnControl.OnLockedOn`
  (params (Active :type Boolean) (TargComponent :type "LockOnTargSceneComponent Object Reference"))
  (`self.LocalSetLockOnAnims` Active)
  (if (`self.IsLocallyControlled`)
    (`self.ServerSetLockOnAnims` Active)))

(event `LocalSetLockOnAnims`
  (params (LockOn :type Boolean))
  (message `/Game/KobWar/CharacterAssets/Kobold/BPI_AnimationChar.SetLockedOn` (`self.AnimInstance`) LockOn))

(event `ServerSetLockOnAnims`
  (params (LockOn :type Boolean))
  (`self.MulticastSetLockOnAnims` LockOn))

(event `MulticastSetLockOnAnims`
  (params (LockOn :type Boolean))
  (if (not (`self.IsLocallyControlled`))
    (`self.LocalSetLockOnAnims` LockOn)))

(event `self.ActionControl.OnToggleAiming`
  (params (Aiming :type Boolean))
  (`self.LocalSetAiming` Aiming))

(event `LocalSetAiming`
  (params (IsAiming :type Boolean))
  (bind _output_get (set `self.IsAiming` IsAiming))
  (`self.SetAiming` _output_get)
  (if (not (`self.HasAuthority`))
    (`self.ServerSetAiming` IsAiming)))

(event `ServerSetAiming`
  (params (IsAiming :type Boolean))
  (bind _output_get (set `self.IsAiming` IsAiming))
  (`self.SetAiming` _output_get))

(event `LocalUpdateAimRot`
  (params (ControlRot :type "Rotator Structure"))
  (bind _output_get (set `self.AimControlRot` ControlRot))
  (if (not (`self.HasAuthority`))
    (`self.ServerUpdateAimRot` _output_get)))

(event `ServerUpdateAimRot`
  (params (ControlRot :type "Rotator Structure"))
  (set `self.AimControlRot` ControlRot))

(fn `InitAnimInstance`
  (bind _returnvalue (`SkeletalMeshComponent.GetAnimInstance` (`self.Mesh`)))
  (`/Engine/EditorBlueprintResources/StandardMacros.IsValid` _returnvalue
    (:`Is Valid`
      (if (`KismetSystemLibrary.DoesImplementInterface` _returnvalue "/Game/KobWar/CharacterAssets/Kobold/BPI_AnimationChar.BPI_AnimationChar_C")
        (set `self.AnimInstance` _returnvalue)))))

(fn `Initialization`
  (`self.InitAnimInstance`)
  (`self.UpdateCosmetics`))

(fn `InterpAimCamStep`
  (params (DeltaTime :type "Float (double-precision)"))
  (bind _interpaim (`self.InterpAim`))
  (bind _cameraboom (`self.CameraBoom`))
  (if (`self.IsLocallyControlled`)
    (if (`self.IsAiming`)
      (if (!= (`self.InterpAim`) 1.0)
        (set `self.InterpAim` (`KismetMathLibrary.FInterpTo` _interpaim 1.0 DeltaTime 5.0))
        (set `SpringArmComponent.TargetArmLength` (`KismetMathLibrary.Lerp` 600.0 400.0 (`self.InterpAim`)) _cameraboom :!label _label)
        (`SceneComponent.K2_SetRelativeLocation` _cameraboom (`KismetMathLibrary.VLerp` (0.0 0.0 70.0) (0.0 70.0 40.0) (`self.InterpAim`)) false false)
        (`CameraComponent.SetFieldOfView` (`self.FollowCamera`) (`KismetMathLibrary.Lerp` 56.0 35.0 (`self.InterpAim`))))
      (elif (!= (`self.InterpAim`) 0.0)
        (set `self.InterpAim` (`KismetMathLibrary.FInterpTo` _interpaim 0.0 DeltaTime 5.0))
        (goto _label)))))

(fn `OnRep_IsAiming`
  (`self.SetAiming` (`self.IsAiming`)))

(fn `SetAiming`
  (params (IsAiming :type Boolean))
  (message `/Game/KobWar/CharacterAssets/Kobold/BPI_AnimationChar.SetAiming` (`self.AnimInstance`) IsAiming)
  (bind _output_get (set `self.bUseControllerRotationYaw` IsAiming))
  (set `CharacterMovementComponent.bOrientRotationToMovement` (not _output_get) (`self.CharacterMovement`)))

(fn `UpdateAimRotStep`
  (params (DeltaTime :type "Float (double-precision)"))
  (if (`self.IsLocallyControlled`)
    (if (`self.IsAiming`)
      (`self.LocalUpdateAimRot` (`self.GetControlRotation`)))))

(fn `UpdateAnimations`
  (params (EquipmentType :type Byte))
  (`/Engine/EditorBlueprintResources/StandardMacros.IsValid` (`self.AnimInstance`)
    (:`Is Valid`
      (message `/Game/KobWar/CharacterAssets/Kobold/BPI_AnimationChar.SetAnimations` (`self.AnimInstance`) EquipmentType))))

(fn `UpdateCosmetics`
  (bind (_gearmesh _bodyoverlaytex _gearmatinst) (`/Game/KobWar/LogicComponents/Appearance/BPFL_GetAppearanceData.LoadCosmetics` (`self.ClassName`) (`self.EquipmentName`) (`self.GenericTeamId`)))
  (`/Game/KobWar/LogicComponents/Appearance/BPC_AppearanceControl.LoadClassGear` (`self.BPC_AppearanceControl`) _gearmesh _bodyoverlaytex _gearmatinst))

(fn `UserConstructionScript`)