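; Input data component that caches action key bindings and tracks whether the player uses keyboard/mouse or gamepad.
; On BeginPlay it builds an action-to-keys map from Input Settings, with two keyboard/mouse slots and gamepad slots, though the second gamepad key overwrites the first.
; AnyKeyPressed broadcasts each key by device and signals mode changes.
; GetInputIcons uses the current mode to return an action's icon textures and text.
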(event `self.ReceiveBeginPlay`
  (`self.LoadMappingsButtons`))

(fn `AnyKeyPressed`
  (params (Key :type "Key Structure" :default "None"))
  (bind _returnvalue (`KismetInputLibrary.Key_IsGamepadKey` Key))
  (bind _returnvalue_2 (or (`KismetInputLibrary.Key_IsMouseButton` Key) (`KismetInputLibrary.Key_IsKeyboardKey` Key)))
  (`|ExecutionSequence`
    (:`then_0`
      (if _returnvalue_2
        (`self.OnAnyKeyboardMouseKey` Key)
        (elif _returnvalue
          (`self.OnAnyGamepadKey` Key))))
    (:`then_1`
      (if (and (not (`self.InKeyboardMode`)) _returnvalue_2)
        (set `self.InKeyboardMode` true)
        (set `self.InGamepadMode` false)
        (`self.OnInputModeChange` true)
        (elif (and (not (`self.InGamepadMode`)) _returnvalue)
          (set `self.InKeyboardMode` false)
          (set `self.InGamepadMode` true)
          (`self.OnInputModeChange` false true))))))

(fn `GetCurrentInputMode`
  (returns (InKeyboardMode :type Boolean) (InGamepadMode :type Boolean))
  (return (`self.InKeyboardMode`) (`self.InGamepadMode`)))

(fn `GetInputIcons`
  (params (InputName :type Name))
  (returns (Texture1 :type "Texture2D Object Reference") (Text1 :type Text) (Texture2 :type "Texture2D Object Reference") (Text2 :type Text))
  (bind (_value _returnvalue) (`BlueprintMapLibrary.Map_Find` (`self.InputMappings`) InputName))
  (bind (_action _keyboardkey1 _keyboardkey2 _gamepadkey1 _gamepadkey2) (break `/Game/KobWar/LogicComponents/Input/Struct_InputMappingData` _value))
  (bind (_texture _text) (`/Game/KobWar/Inputs/BPFL_KeyToIconData.KeyToIconData` _keyboardkey2))
  (bind (_texture_2 _text_2) (`/Game/KobWar/Inputs/BPFL_KeyToIconData.ControllerButtonToIconData` _gamepadkey1))
  (bind (_texture_3 _text_3) (`/Game/KobWar/Inputs/BPFL_KeyToIconData.KeyToIconData` _keyboardkey1))
  (bind (_texture_4 _text_4) (`/Game/KobWar/Inputs/BPFL_KeyToIconData.ControllerButtonToIconData` _gamepadkey2))
  (if _returnvalue
    (if (`self.InKeyboardMode`)
      (return _texture_3 _text_3 _texture _text)
      (elif (`self.InGamepadMode`)
        (return _texture_2 _text_2 _texture_4 _text_4)))))

(fn `LoadMappingsButtons`
  (returns (InputMap :type "Map of Name to /Game/KobWar/LogicComponents/Input/Struct_InputMappingData Structure") (OrderedNames :type "Array of Name"))
  (locals (KeyboardKeysFound :type Byte) (GamepadKeysFound :type Byte) (CurrentInputMappingData :type "/Game/KobWar/LogicComponents/Input/Struct_InputMappingData Structure") (Keyboard1Set :type Boolean) (Keyboard2Set :type Boolean) (Gamepad1Set :type Boolean) (Gamepad2Set :type Boolean) (MappingsOrdered :type "Array of Name"))
  (`BlueprintMapLibrary.Map_Clear` (`self.InputMappings`))
  (bind _output_get (set `local.MappingsOrdered` (`/Game/KobWar/Inputs/BPFL_DefaultKeys.GetActionList`)))
  (for _array_element _output_get
    (set `local.CurrentInputMappingData` (make `/Game/KobWar/LogicComponents/Input/Struct_InputMappingData` _array_element))
    (set `local.Keyboard1Set` false)
    (set `local.Keyboard2Set` false)
    (set `local.Gamepad1Set` false)
    (set `local.Gamepad2Set` false)
    (for _array_element_2 (`InputSettings.GetActionMappingByName` (`InputSettings.GetInputSettings`) _array_element)
      (bind (_actionname _bshift _bctrl _balt _bcmd _key) (break `InputActionKeyMapping` _array_element_2))
      (if (or (`KismetInputLibrary.Key_IsKeyboardKey` _key) (`KismetInputLibrary.Key_IsMouseButton` _key))
        (if (not (`local.Keyboard1Set`))
          (setmembers `/Game/KobWar/LogicComponents/Input/Struct_InputMappingData` :`StructRef` (`local.CurrentInputMappingData`) :`KeyboardKey1` _key)
          (set `local.Keyboard1Set` true)
          (elif (not (`local.Keyboard2Set`))
            (setmembers `/Game/KobWar/LogicComponents/Input/Struct_InputMappingData` :`StructRef` (`local.CurrentInputMappingData`) :`KeyboardKey2` _key)
            (set `local.Keyboard2Set` true)))
        (elif (`KismetInputLibrary.Key_IsGamepadKey` _key)
          (if (not (`local.Gamepad1Set`))
            (setmembers `/Game/KobWar/LogicComponents/Input/Struct_InputMappingData` :`StructRef` (`local.CurrentInputMappingData`) :`GamepadKey1` _key)
            (set `local.Gamepad1Set` true)
            (elif (not (`local.Gamepad2Set`))
              (setmembers `/Game/KobWar/LogicComponents/Input/Struct_InputMappingData` :`StructRef` (`local.CurrentInputMappingData`) :`GamepadKey1` _key)
              (set `local.Gamepad2Set` true))))))
    (`BlueprintMapLibrary.Map_Add` (`self.InputMappings`) _array_element (`local.CurrentInputMappingData`)))
  (return (`self.InputMappings`) (`local.MappingsOrdered`)))