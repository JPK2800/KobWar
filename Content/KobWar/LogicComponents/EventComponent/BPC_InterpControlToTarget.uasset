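; Temporary actor component that eases its owner's control rotation pitch toward a target position, as seen from the owner's follow camera.
; Each tick it interpolates toward the camera-to-target look-at rotation at a set turn speed, applying only pitch and keeping current yaw and roll.
; A timer started on BeginPlay destroys the component once its maximum duration elapses, whether or not the target is reached.
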(event `self.ReceiveBeginPlay`
  (`self.StartDestructTimer`))

(event `self.ReceiveTick`
  (params (DeltaSeconds :type "Float (single-precision)"))
  (`self.RotateStep` DeltaSeconds))

(fn `DestructComponent`
  (bind _destructtimer (`self.DestructTimer`))
  (if (`KismetSystemLibrary.K2_IsValidTimerHandle` _destructtimer)
    (`KismetSystemLibrary.K2_ClearAndInvalidateTimerHandle` _destructtimer)
    (`self.K2_DestroyComponent`)))

(fn `RotateStep`
  (params (Delta :type "Float (double-precision)"))
  (bind _owner (`self.Owner`))
  (bind _returnvalue (`Pawn.GetController` (`self.Owner`)))
  (`/Engine/EditorBlueprintResources/StandardMacros.IsValid` _owner
    (:`Is Valid`
      (`Controller.SetControlRotation` _returnvalue (`KismetMathLibrary.MakeRotator` (.roll (`Controller.GetControlRotation` _returnvalue)) (.pitch (`KismetMathLibrary.RInterpTo` (`Pawn.GetControlRotation` _owner) (`KismetMathLibrary.FindLookAtRotation` (`SceneComponent.K2_GetComponentLocation` (`KobWarCharacter.FollowCamera` _owner)) (`self.TargetPosition`)) Delta (`self.TurnSpeed`))) (.yaw (`Controller.GetControlRotation` _returnvalue)))))))

(fn `StartDestructTimer`
  (bind _returnvalue (`KismetSystemLibrary.K2_SetTimer` self "DestructComponent" (`self.MaxDuration`)))
  (set `self.DestructTimer` _returnvalue))