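; Actor component that smoothly turns its owner toward a target rotation, then destroys itself.
; Each tick, RotateStep applies RInterpTo at TurnSpeed and snaps to TargetRotation once the yaw delta is at most 0.5.
; That delta is signed with no absolute value, so any negative difference snaps immediately.
; A MaxDuration timer started on BeginPlay also triggers DestructComponent, capping the component's lifetime.
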(event `self.ReceiveBeginPlay`
  (`self.StartDestructTimer`))

(event `self.ReceiveTick`
  (params (DeltaSeconds :type "Float (single-precision)"))
  (`self.RotateStep` DeltaSeconds))

(fn `DestructComponent`
  (bind _destructtimer (`self.DestructTimer`))
  (if (`KismetSystemLibrary.K2_IsValidTimerHandle` _destructtimer)
    (`KismetSystemLibrary.K2_ClearAndInvalidateTimerHandle` _destructtimer)
    (`self.K2_DestroyComponent`)))

(fn `RotateStep`
  (params (Delta :type "Float (double-precision)"))
  (bind _owner (`self.Owner`))
  (bind _targetrotation (`self.TargetRotation`))
  (bind _returnvalue (`KismetMathLibrary.RInterpTo` (`Actor.K2_GetActorRotation` _owner) (`self.TargetRotation`) Delta (`self.TurnSpeed`)))
  (`/Engine/EditorBlueprintResources/StandardMacros.IsValid` _owner
    (:`Is Valid`
      (if (<= (.yaw (`KismetMathLibrary.NormalizedDeltaRotator` _returnvalue _targetrotation)) 0.5)
        (`Actor.K2_SetActorRotation` _owner _targetrotation false)
        (`self.DestructComponent`)
        (else
          (`Actor.K2_SetActorRotation` _owner _returnvalue false))))))

(fn `StartDestructTimer`
  (bind _returnvalue (`KismetSystemLibrary.K2_SetTimer` self "DestructComponent" (`self.MaxDuration`)))
  (set `self.DestructTimer` _returnvalue))