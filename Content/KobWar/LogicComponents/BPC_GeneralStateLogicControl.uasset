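; Player character component that turns input, character state, aim and lock-on changes into running, blocking and target-facing behavior.
; Holding the dodge button with enough movement input starts a short timer into running, with tick enabled while held to cancel or restart it.
; Blocking requires Ready state, replicating via server event and RepNotify to the animation interface.
; Lock-on switches rotation to controller yaw while Ready and not running.
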(event `self.ReceiveBeginPlay`
  (`self.InitializeBindings`)
  (`KismetSystemLibrary.K2_SetTimer` null "BeginPlayUpdateBlock" 0.01))

(event `self.ReceiveTick`
  (params (DeltaSeconds :type "Float (single-precision)"))
  (bind _owner (`self.Owner`))
  (if (`self.RunHeld`)
    (`/Engine/EditorBlueprintResources/StandardMacros.IsValid` _owner
      (:`Is Valid`
        (bind _returnvalue (`KobWarCharacter.GetCurrentMovementInput` _owner))
        (`self.RunCheckMoveVal` (`.Y` (`KismetMathLibrary.BreakVector2D` _returnvalue)))))))

(event `ServerSetBlock`
  (params (SetBlocking :type Boolean))
  (bind _output_get (set `self.IsBlocking` SetBlocking))
  (`self.UpdateAnimBlock` _output_get))

(fn `AimToggled`
  (params (Aiming :type Boolean))
  (set `self.IsAiming` Aiming)
  (`|ExecutionSequence`
    (:`then_0`
      (if Aiming
        (`self.RunChargeCancel`)
        (elif (`self.RunHeld`)
          (`self.RunPressed`))))
    (:`then_1`
      (`KobWarCharacter.UpdateSpeed` (`self.Owner`)))))

(fn `BeginPlayUpdateBlock`
  (`self.UpdateAnimBlock` (`self.IsBlocking`)))

(fn `BlockInputReceived`
  (params (Press :type Boolean) (Release :type Boolean))
  (`|ExecutionSequence`
    (:`then_0`
      (if Press
        (`self.BlockPressed`)))
    (:`then_1`
      (if Release
        (`self.BlockReleased`)))))

(fn `BlockPressed`
  (set `self.BlockHeld` true)
  (if (`|EnumEquality` (`self.OwnerState`) "Ready")
    (if (not (`self.IsBlocking`))
      (`self.ServerSetBlock` true)
      (`self.UpdateAnimBlock` true))))

(fn `BlockReleased`
  (set `self.BlockHeld` false)
  (if (`self.IsBlocking`)
    (`self.ServerSetBlock` false)
    (`self.UpdateAnimBlock` false)))

(fn `InitializeBindings`
  (bind _asbp_player_character_base (cast `/Game/KobWar/BP_PlayerCharacterBase` (`self.GetOwner`)))
  (bind _output_get (set `self.Owner` _asbp_player_character_base))
  (add `KobWarCharacter.OnDodgeButton` _asbp_player_character_base (`|CreateDelegate` :!event `RunInputReceived`))
  (add `KobWarCharacter.OnStateChange` _asbp_player_character_base (`|CreateDelegate` :!event `StateChangeReceived`))
  (add `KobWarCharacter.OnBlockButton` _asbp_player_character_base (`|CreateDelegate` :!event `BlockInputReceived`))
  (add `ActionControlComponent.OnToggleAiming` (`KobWarCharacter.ActionControl` _asbp_player_character_base) (`|CreateDelegate` :!event `AimToggled`))
  (add `LockOnComponent.OnLockedOn` (`/Game/KobWar/BP_PlayerCharacterBase.BPC_LockOnControl` _output_get) (`|CreateDelegate` :!event `LockOnChangeReceived`)))

(fn `LockOnChangeReceived`
  (params (Active :type Boolean) (TargComponent :type "LockOnTargSceneComponent Object Reference"))
  (set `self.IsLockedOn` Active)
  (`self.UpdateIfFaceTarget`))

(fn `OnRep_IsBlocking`
  (`self.UpdateAnimBlock` (`self.IsBlocking`)))

(fn `RunBegin`
  (bind _owner (`self.Owner`))
  (set `self.IsRunning` true)
  (set `KobWarCharacter.IsRunning` true _owner)
  (`KobWarCharacter.UpdateSpeed` _owner)
  (`self.UpdateIfFaceTarget`))

(fn `RunChargeCancel`
  (`KismetSystemLibrary.K2_ClearAndInvalidateTimerHandle` (`self.RunTimer`))
  (set `self.RunTimer` (struct))
  (if (`self.IsRunning`)
    (`self.RunEnd`)))

(fn `RunChargeRestart`
  (bind _returnvalue (`KismetSystemLibrary.K2_SetTimer` self "RunBegin" 0.25))
  (set `self.RunTimer` _returnvalue))

(fn `RunCheckMoveVal`
  (params (Value :type "Float (double-precision)"))
  (bind _returnvalue (`KismetMathLibrary.Abs` Value))
  (bind _returnvalue_2 (`KismetSystemLibrary.K2_IsValidTimerHandle` (`self.RunTimer`)))
  (if (`self.RunHeld`)
    (if (and (<= _returnvalue 0.5) _returnvalue_2)
      (`self.RunChargeCancel`)
      (elif (and (>= _returnvalue 0.5) (not _returnvalue_2))
        (if (not (`self.IsAiming`))
          (`self.RunChargeRestart`))))))

(fn `RunEnd`
  (bind _owner (`self.Owner`))
  (set `self.IsRunning` false)
  (set `KobWarCharacter.IsRunning` false _owner)
  (`KobWarCharacter.UpdateSpeed` _owner)
  (`self.UpdateIfFaceTarget`))

(fn `RunInputReceived`
  (params (Press :type Boolean) (Release :type Boolean))
  (`|ExecutionSequence`
    (:`then_0`
      (if Press
        (`self.RunPressed`)))
    (:`then_1`
      (if Release
        (`self.RunReleased`)))))

(fn `RunPressed`
  (set `self.RunHeld` true)
  (`self.SetComponentTickEnabled` true)
  (bind _returnvalue (`KobWarCharacter.GetCurrentMovementInput` (`self.Owner`)))
  (if (and (>= (`.Y` (`KismetMathLibrary.BreakVector2D` _returnvalue)) 0.5) (`|EnumEquality` (`self.OwnerState`) "Ready"))
    (bind _returnvalue_2 (`KismetSystemLibrary.K2_SetTimer` self "RunBegin" 0.25))
    (set `self.RunTimer` _returnvalue_2)))

(fn `RunReleased`
  (set `self.RunHeld` false)
  (`self.SetComponentTickEnabled` false)
  (`KismetSystemLibrary.K2_ClearAndInvalidateTimerHandle` (`self.RunTimer`))
  (if (`self.IsRunning`)
    (`self.RunEnd`)))

(fn `StateChangeReceived`
  (params (NewState :type "ECharacterState Enum" :default "Undefined") (OldState :type "ECharacterState Enum" :default "Undefined"))
  (bind _output_get (set `self.OwnerState` NewState))
  (`|ExecutionSequence`
    (:`then_0`
      (if (and (`|EnumInequality` _output_get "Ready") (`self.RunHeld`))
        (`self.RunChargeCancel`)))
    (:`then_1`
      (if (`|EnumEquality` _output_get "Ready")
        (`|ExecutionSequence`
          (:`then_0`
            (if (`self.RunHeld`)
              (`self.RunPressed`)))
          (:`then_1`
            (if (`self.BlockHeld`)
              (`self.BlockPressed`))))))
    (:`then_2`
      (if (and (`|EnumInequality` _output_get "Ready") (`self.IsRunning`))
        (`self.RunEnd`)))
    (:`then_3`
      (`self.UpdateIfFaceTarget`))
    (:`then_4`)))

(fn `UpdateAnimBlock`
  (params (Toggle :type Boolean))
  (bind _owner (`self.Owner`))
  (bind _animinstance (`/Game/KobWar/BP_PlayerCharacterBase.AnimInstance` _owner))
  (`/Engine/EditorBlueprintResources/StandardMacros.IsValid` _owner
    (:`Is Valid`
      (if (`KismetSystemLibrary.DoesImplementInterface` _animinstance "/Game/KobWar/CharacterAssets/Kobold/BPI_AnimationChar.BPI_AnimationChar_C")
        (message `/Game/KobWar/CharacterAssets/Kobold/BPI_AnimationChar.SetBlocking` _animinstance Toggle)))))

(fn `UpdateIfFaceTarget`
  (locals (ShouldFaceTarget :type Boolean))
  (bind _owner (`self.Owner`))
  (bind _output_get (set `local.ShouldFaceTarget` (and (`self.IsLockedOn`) (`|EnumEquality` (`self.OwnerState`) "Ready") (not (`self.IsRunning`)))))
  (if (!= _output_get (`self.IsFacingTarget`))
    (set `self.IsFacingTarget` _output_get)
    (bind _output_get_2 (set `Pawn.bUseControllerRotationYaw` _output_get _owner))
    (set `CharacterMovementComponent.bOrientRotationToMovement` (not _output_get_2) (`Character.CharacterMovement` _owner))))