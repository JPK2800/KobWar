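; Lock-on control component that shows a target marker widget on the owning player's screen over the locked scene component.
; The lock-on event creates or retargets the widget, and removes it when lock-on ends or the target is invalid.
; Tick interpolates a stored world position toward the target before projecting it, so the marker glides between targets.
; If that position fails to project, interpolation pauses and the widget is hidden through render opacity.
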(event `self.ReceiveBeginPlay`
  (add `self.OnLockedOn` (delegate `OnLockOn`)))

(event `OnLockOn` :!signature `self.OnLockedOn`
  (params (Active :type Boolean) (TargComponent :type "LockOnTargSceneComponent Object Reference"))
  (bind _ownerplayercontroller (`self.OwnerPlayerController`))
  (`/Engine/EditorBlueprintResources/StandardMacros.IsValid` _ownerplayercontroller
    (:`Is Valid`
      (if Active
        (`/Engine/EditorBlueprintResources/StandardMacros.IsValid` TargComponent
          (:`Is Valid`
            (`/Engine/EditorBlueprintResources/StandardMacros.IsValid` (`self.LockOnWidget`)
              (:`Is Valid`
                (`self.SetWidgetOnTarget` (`self.LockOnWidget`) TargComponent))
              (:`Is Not Valid`
                (bind _returnvalue (`|CreateWidget` "/Game/KobWar/LogicComponents/LockOn/WBP_LockOnTarget.WBP_LockOnTarget_C" _ownerplayercontroller))
                (`self.SetWidgetOnTarget` _returnvalue TargComponent true))))
          (:`Is Not Valid`
            (`self.ClearWidgetAndTarget` :!label _label)))
        (else
          (goto _label))))))

(event `self.ReceiveTick`
  (params (DeltaSeconds :type "Float (single-precision)"))
  (`self.InterpWidgetToTargetStep` DeltaSeconds))

(fn `ClearWidgetAndTarget`
  (bind _lockonwidget (`self.LockOnWidget`))
  (set `self.SceneTarg` null)
  (`/Engine/EditorBlueprintResources/StandardMacros.IsValid` _lockonwidget
    (:`Is Valid`
      (`Widget.RemoveFromParent` _lockonwidget))
    (:`Is Not Valid`
      _))
  (set `self.LockOnWidget` null)
  (set `self.IsLockedOn` false))

(fn `InterpWidgetToTargetStep`
  (params (DeltaTime :type "Float (double-precision)"))
  (bind _scenetarg (`self.SceneTarg`))
  (bind _lockonwidget (`self.LockOnWidget`))
  (bind _returnvalue (`Widget.GetRenderOpacity` _lockonwidget))
  (if (`self.IsLockedOn`)
    (`/Engine/EditorBlueprintResources/StandardMacros.IsValid` (`self.LockOnWidget`)
      (:`Is Valid`
        (`/Engine/EditorBlueprintResources/StandardMacros.IsValid` _scenetarg
          (:`Is Valid`
            (bind (_screenposition _returnvalue_2) (`GameplayStatics.ProjectWorldToScreen` (`self.OwnerPlayerController`) (stale _output_get) true))
            (if _returnvalue_2
              (bind _output_get (set `self.WorldPos` (`KismetMathLibrary.VInterpTo` (`self.WorldPos`) (`SceneComponent.K2_GetComponentLocation` _scenetarg) DeltaTime 12.0)))
              (`UserWidget.SetPositionInViewport` _lockonwidget _screenposition true)
              (if (< _returnvalue 0.5)
                (`Widget.SetRenderOpacity` _lockonwidget 1.0))
              (elif (> _returnvalue 0.5)
                (`Widget.SetRenderOpacity` _lockonwidget 0.0)))))))))

(fn `SetWidgetOnTarget`
  (params (LockOnWidget :type "/Game/KobWar/LogicComponents/LockOn/WBP_LockOnTarget Object Reference") (SceneTarg :type "LockOnTargSceneComponent Object Reference") (CreatedWidget :type Boolean))
  (`/Engine/EditorBlueprintResources/StandardMacros.IsValid` LockOnWidget
    (:`Is Valid`
      (`/Engine/EditorBlueprintResources/StandardMacros.IsValid` SceneTarg
        (:`Is Valid`
          (bind _output_get (set `self.LockOnWidget` LockOnWidget))
          (bind _output_get_2 (set `self.SceneTarg` SceneTarg))
          (set `self.IsLockedOn` true)
          (if CreatedWidget
            (bind _returnvalue (`SceneComponent.K2_GetComponentLocation` _output_get_2))
            (set `self.WorldPos` _returnvalue)
            (`UserWidget.SetPositionInViewport` _output_get (`GameplayStatics.ProjectWorldToScreen` (`self.OwnerPlayerController`) _returnvalue true) true)
            (`UserWidget.AddToPlayerScreen` _output_get 0)))))))