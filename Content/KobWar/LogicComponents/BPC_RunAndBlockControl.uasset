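; Player character component that turns held button input into running and blocking, gated by the owner's Ready state.
; It binds to the owner's dodge, block and state-change dispatchers; running starts after a short hold timer and updates owner speed.
; Leaving Ready ends running, and returning resumes held inputs.
; Blocking is set through a server event, with local calls and OnRep updating the animation instance via interface.
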(event `self.ReceiveBeginPlay`
  (`self.InitializeBindings`)
  (`KismetSystemLibrary.K2_SetTimer` null "BeginPlayUpdateBlock" 0.01))

(event `ServerSetBlock`
  (params (SetBlocking :type Boolean))
  (bind _output_get (set `self.IsBlocking` SetBlocking))
  (`self.UpdateAnimBlock` _output_get))

(fn `BeginPlayUpdateBlock`
  (`self.UpdateAnimBlock` (`self.IsBlocking`)))

(fn `BlockInputReceived`
  (params (Press :type Boolean) (Release :type Boolean))
  (`|ExecutionSequence`
    (:`then_0`
      (if Press
        (`self.BlockPressed`)))
    (:`then_1`
      (if Release
        (`self.BlockReleased`)))))

(fn `BlockPressed`
  (set `self.BlockHeld` true)
  (if (`|EnumEquality` (`self.OwnerState`) "Ready")
    (if (not (`self.IsBlocking`))
      (`self.ServerSetBlock` true)
      (`self.UpdateAnimBlock` true))))

(fn `BlockReleased`
  (set `self.BlockHeld` false)
  (if (`self.IsBlocking`)
    (`self.ServerSetBlock` false)
    (`self.UpdateAnimBlock` false)))

(fn `InitializeBindings`
  (bind _asbp_player_character_base (cast `/Game/KobWar/BP_PlayerCharacterBase` (`self.GetOwner`)))
  (set `self.Owner` _asbp_player_character_base)
  (add `KobWarCharacter.OnDodgeButton` _asbp_player_character_base (`|CreateDelegate` :!event `RunInputReceived`))
  (add `KobWarCharacter.OnStateChange` _asbp_player_character_base (`|CreateDelegate` :!event `StateChangeReceived`))
  (add `KobWarCharacter.OnBlockButton` _asbp_player_character_base (`|CreateDelegate` :!event `BlockInputReceived`)))

(fn `OnRep_IsBlocking`
  (`self.UpdateAnimBlock` (`self.IsBlocking`)))

(fn `RunBegin`
  (bind _owner (`self.Owner`))
  (set `self.IsRunning` true)
  (set `KobWarCharacter.IsRunning` true _owner)
  (`KobWarCharacter.UpdateSpeed` _owner)
  (`KismetSystemLibrary.PrintString` "RunBegin"))

(fn `RunEnd`
  (bind _owner (`self.Owner`))
  (set `self.IsRunning` false)
  (set `KobWarCharacter.IsRunning` false _owner)
  (`KobWarCharacter.UpdateSpeed` _owner)
  (`KismetSystemLibrary.PrintString` "RunEnd"))

(fn `RunInputReceived`
  (params (Press :type Boolean) (Release :type Boolean))
  (`|ExecutionSequence`
    (:`then_0`
      (if Press
        (`self.RunPressed`)))
    (:`then_1`
      (if Release
        (`self.RunReleased`)))))

(fn `RunPressed`
  (set `self.RunHeld` true)
  (bind _returnvalue (`KismetSystemLibrary.K2_SetTimer` self "RunBegin" 0.25))
  (set `self.RunTimer` _returnvalue))

(fn `RunReleased`
  (set `self.RunHeld` false)
  (`KismetSystemLibrary.K2_ClearAndInvalidateTimerHandle` (`self.RunTimer`))
  (if (`self.IsRunning`)
    (`self.RunEnd`)))

(fn `StateChangeReceived`
  (params (NewState :type "ECharacterState Enum" :default "Undefined") (OldState :type "ECharacterState Enum" :default "Undefined"))
  (bind _output_get (set `self.OwnerState` NewState))
  (`|ExecutionSequence`
    (:`then_0`
      (if (and (`|EnumInequality` _output_get "Ready") (`self.RunHeld`))
        (`KismetSystemLibrary.K2_ClearAndInvalidateTimerHandle` (`self.RunTimer`))))
    (:`then_1`
      (if (`|EnumEquality` _output_get "Ready")
        (`|ExecutionSequence`
          (:`then_0`
            (if (`self.RunHeld`)
              (`self.RunPressed`)))
          (:`then_1`
            (if (`self.BlockHeld`)
              (`self.BlockPressed`))))))
    (:`then_2`
      (if (and (`|EnumInequality` _output_get "Ready") (`self.IsRunning`))
        (`self.RunEnd`)))))

(fn `UpdateAnimBlock`
  (params (Toggle :type Boolean))
  (bind _owner (`self.Owner`))
  (bind _animinstance (`/Game/KobWar/BP_PlayerCharacterBase.AnimInstance` _owner))
  (`/Engine/EditorBlueprintResources/StandardMacros.IsValid` _owner
    (:`Is Valid`
      (if (`KismetSystemLibrary.DoesImplementInterface` _animinstance "/Game/KobWar/CharacterAssets/Kobold/BPI_AnimationChar.BPI_AnimationChar_C")
        (message `/Game/KobWar/CharacterAssets/Kobold/BPI_AnimationChar.SetBlocking` _animinstance Toggle)))))