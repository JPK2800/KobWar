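; Actor component that manages replicated main-hand and offhand equipment for BP_PlayerCharacterBase.
; The locally controlled owner sends equip data through server events, and the RepNotify on each data variable respawns that slot's actor.
; Spawned items attach to the item_R or item_L mesh socket and get a dynamic material for gear colors.
; All three colors are written to the Color1 parameter, so only the last takes effect.
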(event `self.ReceiveBeginPlay`
  (`self.InitOwner`))

(event `ServerUpdateMainEquip`
  (params (EquipData :type "/Game/KobWar/LogicComponents/Equipment/Struct_EquipmentItemData Structure"))
  (set `self.MainEquipData` EquipData))

(event `ServerUpdateOffhandEquip`
  (params (EquipData :type "/Game/KobWar/LogicComponents/Equipment/Struct_EquipmentItemData Structure"))
  (set `self.OffhandEquipData` EquipData))

(fn `InitOwner`
  (bind _asbp_player_character_base (cast `/Game/KobWar/BP_PlayerCharacterBase` (`self.GetOwner`)))
  (set `self.Owner` _asbp_player_character_base))

(fn `OnRep_MainEquipData`
  (`self.SpawnMainEquipment`))

(fn `OnRep_OffhandEquipData`
  (`self.SpawnOffhandEquipment`))

(fn `SpawnMainEquipment`
  (bind _owner (`self.Owner`))
  (bind (_equipclass _color1 _color2 _color3) (break `/Game/KobWar/LogicComponents/Equipment/Struct_EquipmentItemData` (`self.MainEquipData`)))
  (`|ExecutionSequence`
    (:`then_0`
      (`/Engine/EditorBlueprintResources/StandardMacros.IsValid` (`self.MainEquipment`)
        (:`Is Valid`
          (`Actor.K2_DestroyActor` (`self.MainEquipment`))
          (set `self.MainEquipment` null)
          (set `self.MainEquipmentDynMat` null))))
    (:`then_1`
      (if (`KismetSystemLibrary.IsValidClass` _equipclass)
        (`/Engine/EditorBlueprintResources/StandardMacros.IsValid` _owner
          (:`Is Valid`
            (bind _returnvalue (`|SpawnActorFromClass` _equipclass (`KismetMathLibrary.MakeTransform` (0.0 0.0 0.0)) "Undefined" "OverrideRootScale" null _owner))
            (`Actor.K2_AttachToComponent` _returnvalue (`Character.Mesh` _owner) "item_R" "KeepRelative" "KeepRelative" "KeepWorld" true)
            (bind _output_get (set `self.MainEquipment` _returnvalue))
            (bind _staticmesh (`/Game/KobWar/Equipment/BP_HeldEquipment.StaticMesh` _output_get))
            (bind _returnvalue_2 (`PrimitiveComponent.CreateDynamicMaterialInstance` _staticmesh 0 (`PrimitiveComponent.GetMaterial` _staticmesh 0) "None"))
            (bind _output_get_2 (set `self.MainEquipmentDynMat` _returnvalue_2))
            (bind (_col1 _col2 _col3) (`/Game/KobWar/LogicComponents/Appearance/BPFL_OutfitData.GetGearColors` _color1 _color2 _color3))
            (`MaterialInstanceDynamic.SetVectorParameterValue` _output_get_2 "Color1" _col1)
            (`MaterialInstanceDynamic.SetVectorParameterValue` _output_get_2 "Color1" _col2)
            (`MaterialInstanceDynamic.SetVectorParameterValue` _output_get_2 "Color1" _col3)))))))

(fn `SpawnOffhandEquipment`
  (bind _owner (`self.Owner`))
  (bind (_equipclass _color1 _color2 _color3) (break `/Game/KobWar/LogicComponents/Equipment/Struct_EquipmentItemData` (`self.OffhandEquipData`)))
  (`|ExecutionSequence`
    (:`then_0`
      (`/Engine/EditorBlueprintResources/StandardMacros.IsValid` (`self.OffhandEquipment`)
        (:`Is Valid`
          (`Actor.K2_DestroyActor` (`self.OffhandEquipment`))
          (set `self.OffhandEquipmentDynMat` null)
          (set `self.OffhandEquipmentDynMat` null))))
    (:`then_1`
      (if (`KismetSystemLibrary.IsValidClass` _equipclass)
        (`/Engine/EditorBlueprintResources/StandardMacros.IsValid` _owner
          (:`Is Valid`
            (bind _returnvalue (`|SpawnActorFromClass` _equipclass (`KismetMathLibrary.MakeTransform` (0.0 0.0 0.0)) "Undefined" "OverrideRootScale" null _owner))
            (`Actor.K2_AttachToComponent` _returnvalue (`Character.Mesh` _owner) "item_L" "KeepRelative" "KeepRelative" "KeepWorld" true)
            (bind _output_get (set `self.OffhandEquipment` _returnvalue))
            (bind _staticmesh (`/Game/KobWar/Equipment/BP_HeldEquipment.StaticMesh` _output_get))
            (bind _returnvalue_2 (`PrimitiveComponent.CreateDynamicMaterialInstance` _staticmesh 0 (`PrimitiveComponent.GetMaterial` _staticmesh 0) "None"))
            (bind _output_get_2 (set `self.OffhandEquipmentDynMat` _returnvalue_2))
            (bind (_col1 _col2 _col3) (`/Game/KobWar/LogicComponents/Appearance/BPFL_OutfitData.GetGearColors` _color1 _color2 _color3))
            (`MaterialInstanceDynamic.SetVectorParameterValue` _output_get_2 "Color1" _col1)
            (`MaterialInstanceDynamic.SetVectorParameterValue` _output_get_2 "Color1" _col2)
            (`MaterialInstanceDynamic.SetVectorParameterValue` _output_get_2 "Color1" _col3)))))))

(fn `UpdateMainEquipData`
  (params (EquipData :type "/Game/KobWar/LogicComponents/Equipment/Struct_EquipmentItemData Structure"))
  (`/Engine/EditorBlueprintResources/StandardMacros.IsValid` (`self.Owner`)
    (:`Is Valid`
      _)
    (:`Is Not Valid`
      (`self.InitOwner`)))
  (if (`Pawn.IsLocallyControlled` (`self.Owner`))
    (`self.ServerUpdateMainEquip` EquipData)))

(fn `UpdateOffhandEquipData`
  (params (EquipData :type "/Game/KobWar/LogicComponents/Equipment/Struct_EquipmentItemData Structure"))
  (bind _owner (`self.Owner`))
  (`/Engine/EditorBlueprintResources/StandardMacros.IsValid` _owner
    (:`Is Valid`
      _)
    (:`Is Not Valid`
      (`self.InitOwner`)))
  (if (`Pawn.IsLocallyControlled` _owner)
    (`self.ServerUpdateOffhandEquip` EquipData)))