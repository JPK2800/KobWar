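; Player character component that applies and replicates a kobold's customizable eyes, horns, outfit, headgear and their colors.
; The locally controlled owner loads default debug data, applies it and sends it to server events; others update through BeginPlay and OnRep functions.
; Eye and horn meshes are added as new master-posed components on every update, tinted through dynamic materials.
; Gear colors apply only when that mesh changes, because updates first clear gear materials.
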(event `self.ReceiveBeginPlay`
  (bind _asbp_player_character_base (cast `/Game/KobWar/BP_PlayerCharacterBase` (`self.GetOwner`)))
  (bind _output_get (set `self.Owner` _asbp_player_character_base))
  (if (`Pawn.IsLocallyControlled` _output_get)
    ;[1 1 1] Debug Load
    (`self.LoadAppearanceData` (make `/Game/KobWar/LogicComponents/Appearance/Struct_AppearanceData` 0))
    (`self.LoadOutfitData` (make `/Game/KobWar/LogicComponents/Appearance/Struct_OutfitData` 0))
    (else
      (`self.UpdateAppearanceWithNewData` (`self.AppearanceData`))
      (`self.UpdateOutfitWithNewData` (`self.OutfitData`)))))

(event `ServerUpdateAppearanceData`
  (params (AppearanceData :type "/Game/KobWar/LogicComponents/Appearance/Struct_AppearanceData Structure"))
  (bind _output_get (set `self.AppearanceData` AppearanceData))
  (`self.UpdateAppearanceWithNewData` _output_get))

(event `ServerUpdateOutfitData`
  (params (OutfitData :type "/Game/KobWar/LogicComponents/Appearance/Struct_OutfitData Structure"))
  (bind _output_get (set `self.OutfitData` OutfitData))
  (`self.UpdateOutfitWithNewData` _output_get))

(fn `LoadAppearanceData`
  (params (NewData :type "/Game/KobWar/LogicComponents/Appearance/Struct_AppearanceData Structure"))
  (bind _owner (`self.Owner`))
  (`/Engine/EditorBlueprintResources/StandardMacros.IsValid` _owner
    (:`Is Valid`
      (if (`Pawn.IsLocallyControlled` _owner)
        (`|ExecutionSequence`
          (:`then_0`
            (bind _output_get (set `self.AppearanceData` NewData))
            (`self.UpdateAppearanceWithNewData` _output_get))
          (:`then_1`
            (`self.ServerUpdateAppearanceData` NewData)))))))

(fn `LoadOutfitData`
  (params (OutfitData :type "/Game/KobWar/LogicComponents/Appearance/Struct_OutfitData Structure"))
  (bind _owner (`self.Owner`))
  (`/Engine/EditorBlueprintResources/StandardMacros.IsValid` _owner
    (:`Is Valid`
      (if (`Pawn.IsLocallyControlled` _owner)
        (`|ExecutionSequence`
          (:`then_0`
            (bind _output_get (set `self.OutfitData` OutfitData))
            (`self.UpdateOutfitWithNewData` _output_get))
          (:`then_1`
            (`self.ServerUpdateOutfitData` OutfitData)))))))

(fn `OnRep_AppearanceData`
  (`self.UpdateAppearanceWithNewData` (`self.AppearanceData`)))

(fn `OnRep_OutfitData`
  (`self.UpdateOutfitWithNewData` (`self.OutfitData`)))

(fn `UpdateAppearanceWithNewData`
  (params (AppearanceData :type "/Game/KobWar/LogicComponents/Appearance/Struct_AppearanceData Structure"))
  (bind (_option_eye _option_eyecolor _option_horn _option_horncolor) (break `/Game/KobWar/LogicComponents/Appearance/Struct_AppearanceData` AppearanceData))
  (bind _eyesdynmat (`self.EyesDynMat`))
  (bind _owner (`self.Owner`))
  (bind _horndynmat (`self.HornDynMat`))
  (bind _owner_2 (`self.Owner`))
  (bind _mesh (`Character.Mesh` _owner))
  (bind _mesh_2 (`Character.Mesh` _owner_2))
  (`|ExecutionSequence`
    (:`then_0`
      (bind (_eyematinst _valid) (`/Game/KobWar/LogicComponents/Appearance/BPFL_AppearanceData.GetEyesByIndex` _option_eye))
      (if _valid
        (bind _returnvalue (`|AddComponentByClass` _owner_2 "/Script/Engine.SkeletalMeshComponent" true (`KismetMathLibrary.MakeTransform` (0.0 0.0 0.0))))
        (`SceneComponent.K2_AttachToComponent` _returnvalue _mesh_2 "None" "KeepRelative" "KeepRelative" "KeepRelative" true)
        (`SkinnedMeshComponent.SetSkinnedAssetAndUpdate` _returnvalue "/Game/KobWar/CharacterAssets/Kobold/Eyes/kobold_eyes_model.kobold_eyes_model" true)
        (bind _output_get (set `self.SkeletalMeshEyes` _returnvalue))
        (`SkinnedMeshComponent.SetLeaderPoseComponent` _output_get _mesh_2 false)
        (bind _returnvalue_2 (`PrimitiveComponent.CreateDynamicMaterialInstance` _returnvalue 0 _eyematinst "None"))
        (bind _output_get_2 (set `self.EyesDynMat` _returnvalue_2))
        (`PrimitiveComponent.SetMaterial` _returnvalue 0 _output_get_2)
        (bind (_color1 _color2 _color3) (`/Game/KobWar/LogicComponents/Appearance/BPFL_AppearanceData.GetEyesColors` _option_eyecolor))
        (`MaterialInstanceDynamic.SetVectorParameterValue` _eyesdynmat "Color1" _color1)
        (`MaterialInstanceDynamic.SetVectorParameterValue` _eyesdynmat "Color2" _color2)
        (`MaterialInstanceDynamic.SetVectorParameterValue` _eyesdynmat "Color3" _color3)))
    (:`then_1`
      (bind (_hornmesh _valid_2) (`/Game/KobWar/LogicComponents/Appearance/BPFL_AppearanceData.GetHornsByIndex` _option_horn))
      (if _valid_2
        (bind _returnvalue_3 (`|AddComponentByClass` _owner "/Script/Engine.SkeletalMeshComponent" true (`KismetMathLibrary.MakeTransform` (0.0 0.0 0.0))))
        (`SceneComponent.K2_AttachToComponent` _returnvalue_3 _mesh "None" "KeepRelative" "KeepRelative" "KeepRelative" true)
        (`SkinnedMeshComponent.SetSkinnedAssetAndUpdate` _returnvalue_3 _hornmesh true)
        (bind _output_get_3 (set `self.SkeletalMeshHorns` _returnvalue_3))
        (`SkinnedMeshComponent.SetLeaderPoseComponent` _output_get_3 _mesh false)
        (bind _returnvalue_4 (`PrimitiveComponent.CreateDynamicMaterialInstance` _output_get_3 0 (`PrimitiveComponent.GetMaterial` _output_get_3 0) "None"))
        (bind _output_get_4 (set `self.HornDynMat` _returnvalue_4))
        (`PrimitiveComponent.SetMaterial` _output_get_3 0 _output_get_4)
        (bind (_color1_2 _color2_2 _color3_2) (`/Game/KobWar/LogicComponents/Appearance/BPFL_AppearanceData.GetHornsColor` _option_horncolor))
        (`MaterialInstanceDynamic.SetVectorParameterValue` _horndynmat "Color1" _color1_2)
        (`MaterialInstanceDynamic.SetVectorParameterValue` _horndynmat "Color2" _color2_2)
        (`MaterialInstanceDynamic.SetVectorParameterValue` _horndynmat "Color3" _color3_2)))))

(fn `UpdateOutfitWithNewData`
  (params (OutfitData :type "/Game/KobWar/LogicComponents/Appearance/Struct_OutfitData Structure"))
  (bind (_outfitindex _headindex _gearcolor1 _gearcolor2 _gearcolor3) (break `/Game/KobWar/LogicComponents/Appearance/Struct_OutfitData` OutfitData))
  (bind _skeletalmeshbodygear (`self.SkeletalMeshBodyGear`))
  (bind _skeletalmeshheadgear (`self.SkeletalMeshHeadgear`))
  (bind _bodygeardynmat (`self.BodyGearDynMat`))
  (bind _headgeardynmat (`self.HeadGearDynMat`))
  (`|ExecutionSequence`
    (:`then_0`
      (set `self.BodyGearDynMat` null)
      (set `self.HeadGearDynMat` null))
    (:`then_1`
      (`|ExecutionSequence`
        (:`then_0`
          (bind (_mesh _isvalid) (`/Game/KobWar/LogicComponents/Appearance/BPFL_OutfitData.GetOutfitByIndex` _outfitindex))
          (if _isvalid
            (if (!= _mesh (`SkinnedMeshComponent.SkeletalMesh` (`self.SkeletalMeshBodyGear`)))
              (`SkinnedMeshComponent.SetSkinnedAssetAndUpdate` _skeletalmeshbodygear _mesh true)
              (bind _returnvalue (`PrimitiveComponent.CreateDynamicMaterialInstance` _skeletalmeshbodygear 0 (`PrimitiveComponent.GetMaterial` _skeletalmeshbodygear 0) "None"))
              (bind _output_get (set `self.BodyGearDynMat` _returnvalue))
              (`PrimitiveComponent.SetMaterial` _skeletalmeshbodygear 0 _output_get))))
        (:`then_1`
          (bind (_mesh_2 _isvalid_2) (`/Game/KobWar/LogicComponents/Appearance/BPFL_OutfitData.GetHeadgearByIndex` _headindex))
          (if _isvalid_2
            (if (!= _mesh_2 (`SkinnedMeshComponent.SkeletalMesh` (`self.SkeletalMeshHeadgear`)))
              (`SkinnedMeshComponent.SetSkinnedAssetAndUpdate` _skeletalmeshheadgear _mesh_2 true)
              (bind _returnvalue_2 (`PrimitiveComponent.CreateDynamicMaterialInstance` _skeletalmeshheadgear 0 (`PrimitiveComponent.GetMaterial` _skeletalmeshheadgear 0) "None"))
              (bind _output_get_2 (set `self.HeadGearDynMat` _returnvalue_2))
              (`PrimitiveComponent.SetMaterial` _skeletalmeshheadgear 0 _output_get_2))))
        (:`then_2`
          (bind (_col1 _col2 _col3) (`/Game/KobWar/LogicComponents/Appearance/BPFL_OutfitData.GetGearColors` _gearcolor1 _gearcolor2 _gearcolor3))
          (`|ExecutionSequence`
            (:`then_0`
              (`/Engine/EditorBlueprintResources/StandardMacros.IsValid` _bodygeardynmat
                (:`Is Valid`
                  (`MaterialInstanceDynamic.SetVectorParameterValue` _bodygeardynmat "Color1" _col1)
                  (`MaterialInstanceDynamic.SetVectorParameterValue` _bodygeardynmat "Color2" _col2)
                  (`MaterialInstanceDynamic.SetVectorParameterValue` _bodygeardynmat "Color3" _col3))))
            (:`then_1`
              (`/Engine/EditorBlueprintResources/StandardMacros.IsValid` _headgeardynmat
                (:`Is Valid`
                  (`MaterialInstanceDynamic.SetVectorParameterValue` _headgeardynmat "Color1" _col1)
                  (`MaterialInstanceDynamic.SetVectorParameterValue` _headgeardynmat "Color2" _col2)
                  (`MaterialInstanceDynamic.SetVectorParameterValue` _headgeardynmat "Color3" _col3))))))))))