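; Player controller component that walks the local player through team, class and equipment selection at the start of play.
; An InitializationState step machine, driven by game state rules, opens each selection widget; selections advance it and cancels step it back.
; Spectators exit early through a spectator call, while completion reports the chosen class and equipment.
; Controller menu inputs are relayed to the current widget via BPI_InitMenuInterface.
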(event `self.ReceiveBeginPlay`
  (`self.Initialization`))

(fn `BindToOwnerInputs`
  (bind _ownercontroller (`self.OwnerController`))
  (`/Engine/EditorBlueprintResources/StandardMacros.IsValid` _ownercontroller
    (:`Is Valid`
      (`|ExecutionSequence`
        (:`then_0`
          (add `GamePlayerController.OnMenuConfirm` _ownercontroller (`|CreateDelegate` :!event `OwnerMenuConfirm`))
          (add `GamePlayerController.OnMenuBack` _ownercontroller (`|CreateDelegate` :!event `OwnerMenuBack`))
          (add `GamePlayerController.OnMenuUp` _ownercontroller (`|CreateDelegate` :!event `OwnerMenuUp`))
          (add `GamePlayerController.OnMenuDown` _ownercontroller (`|CreateDelegate` :!event `OwnerMenuDown`))
          (add `GamePlayerController.OnMenuLeft` _ownercontroller (`|CreateDelegate` :!event `OwnerMenuLeft`))
          (add `GamePlayerController.OnMenuRight` _ownercontroller (`|CreateDelegate` :!event `OwnerMenuRight`))
          (add `GamePlayerController.OnMenuMisc1` _ownercontroller (`|CreateDelegate` :!event `OwnerMenuMisc1`))
          (add `GamePlayerController.OnMenuMisc2` _ownercontroller (`|CreateDelegate` :!event `OwnerMenuMisc2`)))))))

(fn `CancelClassSelect`
  (bind _classselectionwidget (`self.ClassSelectionWidget`))
  (if (== (`self.InitializationState`) 2)
    (`|ExecutionSequence`
      (:`then_0`
        (`/Engine/EditorBlueprintResources/StandardMacros.IsValid` _classselectionwidget
          (:`Is Valid`
            (`Widget.RemoveFromParent` _classselectionwidget)
            (set `self.ClassSelectionWidget` null))
          (:`Is Not Valid`
            _))
        (set `self.CurrentWidget` null))
      (:`then_1`
        (set `self.InitializationState` 1)
        (`self.ContinueInitializingProcess`)))))

(fn `CancelEquipmentSelect`
  (bind _equipmentselectionwidget (`self.EquipmentSelectionWidget`))
  (if (== (`self.InitializationState`) 3)
    (`|ExecutionSequence`
      (:`then_0`
        (`/Engine/EditorBlueprintResources/StandardMacros.IsValid` _equipmentselectionwidget
          (:`Is Valid`
            (`Widget.RemoveFromParent` _equipmentselectionwidget)
            (set `self.EquipmentSelectionWidget` null))
          (:`Is Not Valid`
            _))
        (set `self.CurrentWidget` null))
      (:`then_1`
        (set `self.InitializationState` 2)
        (`self.ContinueInitializingProcess`)))))

(fn `CancelSpectating`
  (set `self.InitializationState` 1)
  (`self.ContinueInitializingProcess`))

(fn `ContinueInitializingProcess`
  (bind _initializationstate (`self.InitializationState`))
  (bind _ownercontroller (`self.OwnerController`))
  (bind (_charclassname _skeleton) (break `PlayableClassStruct` (`self.ClassDataSelected`)))
  (if (== _initializationstate 0)
    (return)
    (elif (and (== _initializationstate 1) (`self.RequiresTeamSelection`))
      (`self.CreateTeamSelectionWidget`)
      (return)
      (elif (and (>= (`self.InitializationState`) 2) (== (`self.TeamSelected`) (enumliteral `ETeam` "Spectating")))
        (`self.SpectatorTeamSet`)
        (return)
        (elif (and (== _initializationstate 2) (`self.RequiresClassSelection`))
          (`self.CreateClassSelectionWidget`)
          (return)
          (elif (and (== _initializationstate 3) (`self.RequiresClassSelection`))
            (`self.CreateEquipmentSelectionWidget`)
            (return)
            (elif (== _initializationstate 4)
              (set `PlayerController.bShowMouseCursor` false _ownercontroller)
              (`/Game/KobWar/Controllers/BP_PlayerController.UnpauseCharacterInputsForMenu` _ownercontroller)
              (`self.ClassEquipmentSet` _charclassname (`self.SelectedEquipment`) _skeleton)
              (`KismetSystemLibrary.CollectGarbage`))))))))

(fn `CreateClassSelectionWidget`
  (bind _ownercontroller (`self.OwnerController`))
  (bind _classselectionwidget (`self.ClassSelectionWidget`))
  (`/Engine/EditorBlueprintResources/StandardMacros.IsValid` _ownercontroller
    (:`Is Valid`
      (`/Engine/EditorBlueprintResources/StandardMacros.IsValid` (`self.GameState`)
        (:`Is Valid`
          (`/Engine/EditorBlueprintResources/StandardMacros.IsValid` (`self.ClassSelectionWidget`)
            (:`Is Valid`
              (`/Game/KobWar/GameModeLogic/ClassSelection/WBP_ClassSelectionWidget.ToggleInputs` _classselectionwidget true)
              (set `self.CurrentWidget` _classselectionwidget))
            (:`Is Not Valid`
              (bind _returnvalue (`|CreateWidget` "/Game/KobWar/GameModeLogic/ClassSelection/WBP_ClassSelectionWidget.WBP_ClassSelectionWidget_C" _ownercontroller self))
              (`/Game/KobWar/GameModeLogic/ClassSelection/WBP_ClassSelectionWidget.Init1ClassOptions` _returnvalue (`/Game/KobWar/GameModeLogic/BP_GameState.PlayableClasses` (`self.GameState`)))
              (`UserWidget.AddToPlayerScreen` _returnvalue 0)
              (bind _output_get (set `self.ClassSelectionWidget` _returnvalue))
              (set `PlayerController.bShowMouseCursor` true _ownercontroller)
              (set `self.CurrentWidget` _output_get))))))))

(fn `CreateEquipmentSelectionWidget`
  (bind _ownercontroller (`self.OwnerController`))
  (`/Engine/EditorBlueprintResources/StandardMacros.IsValid` _ownercontroller
    (:`Is Valid`
      (`/Engine/EditorBlueprintResources/StandardMacros.IsValid` (`self.GameState`)
        (:`Is Valid`
          (`/Game/KobWar/GameModeLogic/ClassSelection/WBP_ClassSelectionWidget.ToggleInputs` (`self.ClassSelectionWidget`) false)
          (bind _returnvalue (`|CreateWidget` "/Game/KobWar/GameModeLogic/EquipmentSelection/WBP_EquipmentSelectionWidget.WBP_EquipmentSelectionWidget_C" _ownercontroller self))
          (`UserWidget.SetPositionInViewport` _returnvalue (`self.ClassSelectedScreenPos`) true)
          (`/Game/KobWar/GameModeLogic/EquipmentSelection/WBP_EquipmentSelectionWidget.Init1EquipmentOptions` _returnvalue (`.Equipment` (break `PlayableClassStruct` (`self.ClassDataSelected`))))
          (`UserWidget.AddToPlayerScreen` _returnvalue 0)
          (bind _output_get (set `self.EquipmentSelectionWidget` _returnvalue))
          (set `PlayerController.bShowMouseCursor` true _ownercontroller)
          (set `self.CurrentWidget` _output_get))))))

(fn `CreateTeamSelectionWidget`
  (bind _ownercontroller (`self.OwnerController`))
  (`/Engine/EditorBlueprintResources/StandardMacros.IsValid` _ownercontroller
    (:`Is Valid`
      (`|ExecutionSequence`
        (:`then_0`
          (bind _returnvalue (`|CreateWidget` "/Game/KobWar/GameModeLogic/TeamSelection/WBP_TeamSelectionWidget.WBP_TeamSelectionWidget_C" _ownercontroller self))
          (`UserWidget.AddToPlayerScreen` _returnvalue 0)
          (bind _output_get (set `self.TeamSelectionWidget` _returnvalue))
          (set `PlayerController.bShowMouseCursor` true _ownercontroller)
          (set `self.CurrentWidget` _output_get))))))

(fn `Initialization`
  (bind _asbp_player_controller (cast `/Game/KobWar/Controllers/BP_PlayerController` (`self.GetOwner`)))
  (if (`Controller.IsLocalPlayerController` _asbp_player_controller)
    (set `self.OwnerController` _asbp_player_controller)
    (`self.BindToOwnerInputs`)
    (`self.LoadGameModeData`)
    (set `self.InitializationState` 1)
    (`self.ContinueInitializingProcess`)))

(fn `LoadGameModeData`
  (bind _asbp_game_state (cast `/Game/KobWar/GameModeLogic/BP_GameState` (`GameplayStatics.GetGameState`)))
  (bind _output_get (set `self.GameState` _asbp_game_state))
  (set `self.RequiresTeamSelection` (and (`/Game/KobWar/GameModeLogic/BP_GameState.IsTeamBased` _output_get) (`/Game/KobWar/GameModeLogic/BP_GameState.AllowTeamSelection` _output_get)))
  (set `self.RequiresClassSelection` (`/Game/KobWar/GameModeLogic/BP_GameState.AllowClassSelection` _asbp_game_state))
  (bind _playableclasses (`/Game/KobWar/GameModeLogic/BP_GameState.PlayableClasses` _asbp_game_state))
  (if (>= (`KismetArrayLibrary.Array_Length` _playableclasses) 1)
    (bind _output (`|GetArrayItem` _playableclasses))
    (set `self.ClassDataSelected` _output)
    (bind (_charclassname _skeleton _equipment) (break `PlayableClassStruct` _output))
    (if (>= (`KismetArrayLibrary.Array_Length` _equipment) 1)
      (set `self.SelectedEquipment` (`|GetArrayItem` _equipment)))))

(fn `OwnerMenuBack`
  (params (Press :type Boolean) (Release :type Boolean))
  (bind _currentwidget (`self.CurrentWidget`))
  (`/Engine/EditorBlueprintResources/StandardMacros.IsValid` _currentwidget
    (:`Is Valid`
      (if (`KismetSystemLibrary.DoesImplementInterface` _currentwidget "/Game/KobWar/Menus/MainMenuInterfaces/BPI_InitMenuInterface.BPI_InitMenuInterface_C")
        (message `/Game/KobWar/Menus/MainMenuInterfaces/BPI_InitMenuInterface.MenuBackInput` _currentwidget Press Release)))))

(fn `OwnerMenuConfirm`
  (params (Press :type Boolean) (Release :type Boolean))
  (bind _currentwidget (`self.CurrentWidget`))
  (`/Engine/EditorBlueprintResources/StandardMacros.IsValid` _currentwidget
    (:`Is Valid`
      (if (`KismetSystemLibrary.DoesImplementInterface` _currentwidget "/Game/KobWar/Menus/MainMenuInterfaces/BPI_InitMenuInterface.BPI_InitMenuInterface_C")
        (message `/Game/KobWar/Menus/MainMenuInterfaces/BPI_InitMenuInterface.MenuConfirmInput` _currentwidget Press Release)))))

(fn `OwnerMenuDown`
  (params (Press :type Boolean) (Release :type Boolean))
  (bind _currentwidget (`self.CurrentWidget`))
  (`/Engine/EditorBlueprintResources/StandardMacros.IsValid` _currentwidget
    (:`Is Valid`
      (if (`KismetSystemLibrary.DoesImplementInterface` _currentwidget "/Game/KobWar/Menus/MainMenuInterfaces/BPI_InitMenuInterface.BPI_InitMenuInterface_C")
        (message `/Game/KobWar/Menus/MainMenuInterfaces/BPI_InitMenuInterface.MenuDownInput` _currentwidget Press Release)))))

(fn `OwnerMenuLeft`
  (params (Press :type Boolean) (Release :type Boolean))
  (bind _currentwidget (`self.CurrentWidget`))
  (`/Engine/EditorBlueprintResources/StandardMacros.IsValid` _currentwidget
    (:`Is Valid`
      (if (`KismetSystemLibrary.DoesImplementInterface` _currentwidget "/Game/KobWar/Menus/MainMenuInterfaces/BPI_InitMenuInterface.BPI_InitMenuInterface_C")
        (message `/Game/KobWar/Menus/MainMenuInterfaces/BPI_InitMenuInterface.MenuLeftInput` _currentwidget Press Release)))))

(fn `OwnerMenuMisc1`
  (params (Press :type Boolean) (Release :type Boolean))
  (bind _currentwidget (`self.CurrentWidget`))
  (`/Engine/EditorBlueprintResources/StandardMacros.IsValid` _currentwidget
    (:`Is Valid`
      (if (`KismetSystemLibrary.DoesImplementInterface` _currentwidget "/Game/KobWar/Menus/MainMenuInterfaces/BPI_InitMenuInterface.BPI_InitMenuInterface_C")
        (message `/Game/KobWar/Menus/MainMenuInterfaces/BPI_InitMenuInterface.MenuMisc1Input` _currentwidget Press Release)))))

(fn `OwnerMenuMisc2`
  (params (Press :type Boolean) (Release :type Boolean))
  (bind _currentwidget (`self.CurrentWidget`))
  (`/Engine/EditorBlueprintResources/StandardMacros.IsValid` _currentwidget
    (:`Is Valid`
      (if (`KismetSystemLibrary.DoesImplementInterface` _currentwidget "/Game/KobWar/Menus/MainMenuInterfaces/BPI_InitMenuInterface.BPI_InitMenuInterface_C")
        (message `/Game/KobWar/Menus/MainMenuInterfaces/BPI_InitMenuInterface.MenuMisc2Input` _currentwidget Press Release)))))

(fn `OwnerMenuRight`
  (params (Press :type Boolean) (Release :type Boolean))
  (bind _currentwidget (`self.CurrentWidget`))
  (`/Engine/EditorBlueprintResources/StandardMacros.IsValid` _currentwidget
    (:`Is Valid`
      (if (`KismetSystemLibrary.DoesImplementInterface` _currentwidget "/Game/KobWar/Menus/MainMenuInterfaces/BPI_InitMenuInterface.BPI_InitMenuInterface_C")
        (message `/Game/KobWar/Menus/MainMenuInterfaces/BPI_InitMenuInterface.MenuRightInput` _currentwidget Press Release)))))

(fn `OwnerMenuUp`
  (params (Press :type Boolean) (Release :type Boolean))
  (bind _currentwidget (`self.CurrentWidget`))
  (`/Engine/EditorBlueprintResources/StandardMacros.IsValid` _currentwidget
    (:`Is Valid`
      (if (`KismetSystemLibrary.DoesImplementInterface` _currentwidget "/Game/KobWar/Menus/MainMenuInterfaces/BPI_InitMenuInterface.BPI_InitMenuInterface_C")
        (message `/Game/KobWar/Menus/MainMenuInterfaces/BPI_InitMenuInterface.MenuUpInput` _currentwidget Press Release)))))

(fn `UpdateClassSelected`
  (params (Class :type "PlayableClassStruct Structure (by ref)") (EquipmentName :type Name) (ClassSelectedScreenPos :type "Vector2D Structure"))
  (set `self.SelectedEquipment` EquipmentName)
  (set `self.ClassDataSelected` Class)
  (set `self.ClassSelectedScreenPos` ClassSelectedScreenPos)
  (if (< (`self.InitializationState`) 3)
    (set `self.InitializationState` 3))
  (`self.ContinueInitializingProcess`))

(fn `UpdateEquipmentSelected`
  (params (Equipment :type Name))
  (bind _classselectionwidget (`self.ClassSelectionWidget`))
  (bind _equipmentselectionwidget (`self.EquipmentSelectionWidget`))
  (set `self.SelectedEquipment` Equipment)
  (if (<= (`self.InitializationState`) 3)
    (set `self.InitializationState` 4))
  (`|ExecutionSequence`
    (:`then_0`
      (`/Engine/EditorBlueprintResources/StandardMacros.IsValid` _classselectionwidget
        (:`Is Valid`
          (`Widget.RemoveFromParent` _classselectionwidget)
          (set `self.ClassSelectionWidget` null))))
    (:`then_1`
      (`/Engine/EditorBlueprintResources/StandardMacros.IsValid` _equipmentselectionwidget
        (:`Is Valid`
          (`Widget.RemoveFromParent` _equipmentselectionwidget)
          (set `self.EquipmentSelectionWidget` null))))
    (:`then_2`
      (set `self.CurrentWidget` null))
    (:`then_3`
      (`self.ContinueInitializingProcess`))))

(fn `UpdateTeamSelected`
  (params (TeamSelected :type Byte))
  (bind _teamselectionwidget (`self.TeamSelectionWidget`))
  (`|ExecutionSequence`
    (:`then_0`
      (if (or (!= (`self.TeamSelected`) TeamSelected) (== TeamSelected 0))
        (set `self.TeamSelected` TeamSelected)
        (else
          (`/Engine/EditorBlueprintResources/StandardMacros.IsValid` _teamselectionwidget :!label _label
            (:`Is Valid`
              (`Widget.RemoveFromParent` _teamselectionwidget)
              (set `self.TeamSelectionWidget` null)
              (set `self.CurrentWidget` null)
              (set `PlayerController.bShowMouseCursor` false (`self.OwnerController`)))
            (:`Is Not Valid`
              _))
          (`self.ContinueInitializingProcess`))))
    (:`then_1`
      (if (< (`self.InitializationState`) 3)
        (if (`self.RequiresClassSelection`)
          (set `self.InitializationState` 2)
          (goto _label)
          (else
            (set `self.InitializationState` 4)
            (goto _label)))
        (else
          (goto _label))))))