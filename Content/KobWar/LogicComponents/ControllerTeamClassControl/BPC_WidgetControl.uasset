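; Player controller component that walks the local player through team and class selection screens.
; It reads the game mode's rules on BeginPlay, then an InitializationState counter decides whether to show the team widget, the class widget or switch to game-only input.
; The widgets receive the component as a reference, and its update functions store picks, close the screen and advance the state.
; Controller menu inputs are forwarded to the current widget through BPI_MenuMainInterface.
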(event `self.ReceiveBeginPlay`
  (`self.Initialization`))

(fn `BindToOwnerInputs`
  (bind _ownercontroller (`self.OwnerController`))
  (`/Engine/EditorBlueprintResources/StandardMacros.IsValid` _ownercontroller
    (:`Is Valid`
      (add `GamePlayerController.OnMenuConfirm` _ownercontroller (`|CreateDelegate` :!event `OwnerMenuConfirm`))
      (add `GamePlayerController.OnMenuBack` _ownercontroller (`|CreateDelegate` :!event `OwnerMenuBack`))
      (add `GamePlayerController.OnMenuUp` _ownercontroller (`|CreateDelegate` :!event `OwnerMenuUp`))
      (add `GamePlayerController.OnMenuDown` _ownercontroller (`|CreateDelegate` :!event `OwnerMenuDown`))
      (add `GamePlayerController.OnMenuLeft` _ownercontroller (`|CreateDelegate` :!event `OwnerMenuLeft`))
      (add `GamePlayerController.OnMenuRight` _ownercontroller (`|CreateDelegate` :!event `OwnerMenuRight`))
      (add `GamePlayerController.OnMenuMisc1` _ownercontroller (`|CreateDelegate` :!event `OwnerMenuMisc1`))
      (add `GamePlayerController.OnMenuMisc2` _ownercontroller (`|CreateDelegate` :!event `OwnerMenuMisc2`)))))

(fn `ContinueInitializingProcess`
  (bind _initializationstate (`self.InitializationState`))
  (if (== _initializationstate 0)
    (return)
    (elif (and (== _initializationstate 1) (`self.RequiresTeamSelection`))
      (`self.CreateTeamSelectionWidget`)
      (return)
      (elif (and (== _initializationstate 2) (`self.RequiresClassSelection`))
        (`self.CreateClassSelectionWidget`)
        (return)
        (else
          (`WidgetBlueprintLibrary.SetInputMode_GameOnly` (`self.OwnerController`)))))))

(fn `CreateClassSelectionWidget`
  (bind _ownercontroller (`self.OwnerController`))
  (bind _gamemode (`self.GameMode`))
  (`/Engine/EditorBlueprintResources/StandardMacros.IsValid` _ownercontroller
    (:`Is Valid`
      (`/Engine/EditorBlueprintResources/StandardMacros.IsValid` _gamemode
        (:`Is Valid`
          (bind _returnvalue (`|CreateWidget` "/Game/KobWar/GameModeLogic/ClassSelection/WBP_ClassSelectionWidget.WBP_ClassSelectionWidget_C" _ownercontroller self))
          (`/Game/KobWar/GameModeLogic/ClassSelection/WBP_ClassSelectionWidget.UpdateClassOptions` _returnvalue (`KobWarGameMode.PlayableClasses` _gamemode))
          (`UserWidget.AddToPlayerScreen` _returnvalue 0)
          (bind _output_get (set `self.ClassSelectionWidget` _returnvalue))
          (set `PlayerController.bShowMouseCursor` true _ownercontroller)
          (set `self.CurrentWidget` _output_get))))))

(fn `CreateTeamSelectionWidget`
  (bind _ownercontroller (`self.OwnerController`))
  (`/Engine/EditorBlueprintResources/StandardMacros.IsValid` _ownercontroller
    (:`Is Valid`
      (`|ExecutionSequence`
        (:`then_0`
          (bind _returnvalue (`|CreateWidget` "/Game/KobWar/GameModeLogic/TeamSelection/WBP_TeamSelectionWidget.WBP_TeamSelectionWidget_C" _ownercontroller self))
          (`UserWidget.AddToPlayerScreen` _returnvalue 0)
          (bind _output_get (set `self.TeamSelectionWidget` _returnvalue))
          (set `PlayerController.bShowMouseCursor` true _ownercontroller)
          (set `self.CurrentWidget` _output_get))))))

(fn `Initialization`
  (bind _asbp_player_controller (cast `/Game/KobWar/Controllers/BP_PlayerController` (`self.GetOwner`)))
  (if (`Controller.IsLocalController` _asbp_player_controller)
    (set `self.OwnerController` _asbp_player_controller)
    (`self.BindToOwnerInputs`)
    (`self.LoadGameModeData`)
    (set `self.InitializationState` 1)
    (`self.ContinueInitializingProcess`)))

(fn `LoadGameModeData`
  (bind _asbp_base_game_mode (cast `/Game/KobWar/GameModeLogic/BP_BaseGameMode` (`GameplayStatics.GetGameMode`)))
  (bind _output_get (set `self.GameMode` _asbp_base_game_mode))
  (set `self.RequiresTeamSelection` (and (`KobWarGameMode.IsTeamBased` _output_get) (`KobWarGameMode.AllowTeamSelection` _output_get)))
  (set `self.RequiresClassSelection` (`KobWarGameMode.AllowClassSelection` _output_get)))

(fn `OwnerMenuBack`
  (params (Press :type Boolean) (Release :type Boolean))
  (bind _currentwidget (`self.CurrentWidget`))
  (`/Engine/EditorBlueprintResources/StandardMacros.IsValid` _currentwidget
    (:`Is Valid`
      (if (`KismetSystemLibrary.DoesImplementInterface` _currentwidget "/Game/KobWar/Menus/BPI_MenuMainInterface.BPI_MenuMainInterface_C")
        (message `/Game/KobWar/Menus/BPI_MenuMainInterface.MenuBackInput` _currentwidget Press Release)))))

(fn `OwnerMenuConfirm`
  (params (Press :type Boolean) (Release :type Boolean))
  (bind _currentwidget (`self.CurrentWidget`))
  (`/Engine/EditorBlueprintResources/StandardMacros.IsValid` _currentwidget
    (:`Is Valid`
      (if (`KismetSystemLibrary.DoesImplementInterface` _currentwidget "/Game/KobWar/Menus/BPI_MenuMainInterface.BPI_MenuMainInterface_C")
        (message `/Game/KobWar/Menus/BPI_MenuMainInterface.MenuConfirmInput` _currentwidget Press Release)))))

(fn `OwnerMenuDown`
  (params (Press :type Boolean) (Release :type Boolean))
  (bind _currentwidget (`self.CurrentWidget`))
  (`/Engine/EditorBlueprintResources/StandardMacros.IsValid` _currentwidget
    (:`Is Valid`
      (if (`KismetSystemLibrary.DoesImplementInterface` _currentwidget "/Game/KobWar/Menus/BPI_MenuMainInterface.BPI_MenuMainInterface_C")
        (message `/Game/KobWar/Menus/BPI_MenuMainInterface.MenuDownInput` _currentwidget Press Release)))))

(fn `OwnerMenuLeft`
  (params (Press :type Boolean) (Release :type Boolean))
  (bind _currentwidget (`self.CurrentWidget`))
  (`/Engine/EditorBlueprintResources/StandardMacros.IsValid` _currentwidget
    (:`Is Valid`
      (if (`KismetSystemLibrary.DoesImplementInterface` _currentwidget "/Game/KobWar/Menus/BPI_MenuMainInterface.BPI_MenuMainInterface_C")
        (message `/Game/KobWar/Menus/BPI_MenuMainInterface.MenuLeftInput` _currentwidget Press Release)))))

(fn `OwnerMenuMisc1`
  (params (Press :type Boolean) (Release :type Boolean))
  (bind _currentwidget (`self.CurrentWidget`))
  (`/Engine/EditorBlueprintResources/StandardMacros.IsValid` _currentwidget
    (:`Is Valid`
      (if (`KismetSystemLibrary.DoesImplementInterface` _currentwidget "/Game/KobWar/Menus/BPI_MenuMainInterface.BPI_MenuMainInterface_C")
        (message `/Game/KobWar/Menus/BPI_MenuMainInterface.MenuMisc1Input` _currentwidget Press Release)))))

(fn `OwnerMenuMisc2`
  (params (Press :type Boolean) (Release :type Boolean))
  (bind _currentwidget (`self.CurrentWidget`))
  (`/Engine/EditorBlueprintResources/StandardMacros.IsValid` _currentwidget
    (:`Is Valid`
      (if (`KismetSystemLibrary.DoesImplementInterface` _currentwidget "/Game/KobWar/Menus/BPI_MenuMainInterface.BPI_MenuMainInterface_C")
        (message `/Game/KobWar/Menus/BPI_MenuMainInterface.MenuMisc2Input` _currentwidget Press Release)))))

(fn `OwnerMenuRight`
  (params (Press :type Boolean) (Release :type Boolean))
  (bind _currentwidget (`self.CurrentWidget`))
  (`/Engine/EditorBlueprintResources/StandardMacros.IsValid` _currentwidget
    (:`Is Valid`
      (if (`KismetSystemLibrary.DoesImplementInterface` _currentwidget "/Game/KobWar/Menus/BPI_MenuMainInterface.BPI_MenuMainInterface_C")
        (message `/Game/KobWar/Menus/BPI_MenuMainInterface.MenuRightInput` _currentwidget Press Release)))))

(fn `OwnerMenuUp`
  (params (Press :type Boolean) (Release :type Boolean))
  (bind _currentwidget (`self.CurrentWidget`))
  (`/Engine/EditorBlueprintResources/StandardMacros.IsValid` _currentwidget
    (:`Is Valid`
      (if (`KismetSystemLibrary.DoesImplementInterface` _currentwidget "/Game/KobWar/Menus/BPI_MenuMainInterface.BPI_MenuMainInterface_C")
        (message `/Game/KobWar/Menus/BPI_MenuMainInterface.MenuUpInput` _currentwidget Press Release)))))

(fn `UpdateClassSelected`
  (params (Class :type "PlayableClassStruct Structure (by ref)") (EquipmentName :type Name))
  (bind _classselectionwidget (`self.ClassSelectionWidget`))
  (bind _classdataselected_charclassname (break `PlayableClassStruct` (`self.ClassDataSelected`)))
  (if (!= (`.CharClassName` (break `PlayableClassStruct` Class)) _classdataselected_charclassname)
    (set `self.SelectedEquipment` EquipmentName)
    (set `self.ClassDataSelected` Class)
    (if (< (`self.TeamSelected`) 3)
      (set `self.InitializationState` 3))
    (`/Engine/EditorBlueprintResources/StandardMacros.IsValid` _classselectionwidget
      (:`Is Valid`
        (`Widget.RemoveFromParent` _classselectionwidget)
        (set `self.ClassSelectionWidget` null)
        (set `self.CurrentWidget` null)
        (set `PlayerController.bShowMouseCursor` false (`self.OwnerController`)))
      (:`Is Not Valid`
        _))
    (`self.ContinueInitializingProcess`)))

(fn `UpdateTeamSelected`
  (params (TeamSelected :type Byte))
  (bind _teamselectionwidget (`self.TeamSelectionWidget`))
  (if (!= (`self.TeamSelected`) TeamSelected)
    (set `self.TeamSelected` TeamSelected)
    (if (< (`self.TeamSelected`) 3)
      (set `self.InitializationState` 2))
    (`/Engine/EditorBlueprintResources/StandardMacros.IsValid` _teamselectionwidget
      (:`Is Valid`
        (`Widget.RemoveFromParent` _teamselectionwidget)
        (set `self.TeamSelectionWidget` null)
        (set `self.CurrentWidget` null)
        (set `PlayerController.bShowMouseCursor` false (`self.OwnerController`)))
      (:`Is Not Valid`
        _))
    (`self.ContinueInitializingProcess`)))