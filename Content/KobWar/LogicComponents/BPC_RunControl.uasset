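; Actor component that adds hold-to-run to BP_PlayerCharacterBase, driven by the owner's dodge button and state changes.
; Holding the button starts a short timer before running begins; release cancels it or ends the run.
; Leaving the Ready state cancels or stops running, and returning to Ready while held restarts the timer.
; Run changes set the owner's IsRunning flag and call UpdateSpeed.
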(event `self.ReceiveBeginPlay`
  (`self.InitializeBindings`))

(fn `InitializeBindings`
  (bind _asbp_player_character_base (cast `/Game/KobWar/BP_PlayerCharacterBase` (`self.GetOwner`)))
  (set `self.Owner` _asbp_player_character_base)
  (add `KobWarCharacter.OnDodgeButton` _asbp_player_character_base (`|CreateDelegate` :!event `RunInputReceived`))
  (add `KobWarCharacter.OnStateChange` _asbp_player_character_base (`|CreateDelegate` :!event `StateChangeReceived`)))

(fn `RunBegin`
  (bind _owner (`self.Owner`))
  (set `self.IsRunning` true)
  (set `KobWarCharacter.IsRunning` true _owner)
  (`KobWarCharacter.UpdateSpeed` _owner)
  (`KismetSystemLibrary.PrintString` "RunBegin"))

(fn `RunEnd`
  (bind _owner (`self.Owner`))
  (set `self.IsRunning` false)
  (set `KobWarCharacter.IsRunning` false _owner)
  (`KobWarCharacter.UpdateSpeed` _owner)
  (`KismetSystemLibrary.PrintString` "RunEnd"))

(fn `RunInputReceived`
  (params (Press :type Boolean) (Release :type Boolean))
  (`|ExecutionSequence`
    (:`then_0`
      (if Press
        (`self.RunPressed`)
        (`KismetSystemLibrary.PrintString` "RunPressed")))
    (:`then_1`
      (if Release
        (`self.RunReleased`)
        (`KismetSystemLibrary.PrintString` "RunReleased")))))

(fn `RunPressed`
  (set `self.RunHeld` true)
  (bind _returnvalue (`KismetSystemLibrary.K2_SetTimer` self "RunBegin" 0.25))
  (set `self.RunTimer` _returnvalue))

(fn `RunReleased`
  (set `self.RunHeld` false)
  (`KismetSystemLibrary.K2_ClearAndInvalidateTimerHandle` (`self.RunTimer`))
  (if (`self.IsRunning`)
    (`self.RunEnd`)))

(fn `StateChangeReceived`
  (params (NewState :type "ECharacterState Enum" :default "Undefined") (OldState :type "ECharacterState Enum" :default "Undefined"))
  (bind _output_get (set `self.OwnerState` NewState))
  (`|ExecutionSequence`
    (:`then_0`
      (if (and (`|EnumInequality` _output_get "Ready") (`self.RunHeld`))
        (`KismetSystemLibrary.K2_ClearAndInvalidateTimerHandle` (`self.RunTimer`))))
    (:`then_1`
      (if (and (`|EnumEquality` _output_get "Ready") (`self.RunHeld`))
        (`self.RunPressed`)))
    (:`then_2`
      (if (and (`|EnumInequality` _output_get "Ready") (`self.IsRunning`))
        (`self.RunEnd`)))))