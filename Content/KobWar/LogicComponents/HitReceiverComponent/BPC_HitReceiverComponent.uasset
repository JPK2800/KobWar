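; Actor component that handles incoming hits on a BP_PlayerCharacterBase owner, turning it toward the attacker and forcing a stagger unless the hit was dodged.
; Hits enter on the locally controlled client and relay through server and multicast events, but TakeHit only reacts where the owner is locally controlled.
; The resulting yaw change is applied locally at once, then propagated through its own server and multicast chain, skipping the controlling client on multicast.
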(event `self.ReceiveBeginPlay`
  (`self.InitOwner`))

(event `LocalTakeHit`
  (params (Data :type "/Game/KobWar/LogicComponents/HitReceiverComponent/Struct_TakeHitData Structure"))
  (if (`Pawn.IsLocallyControlled` (`self.Owner`))
    (`self.ServerTakeHit` Data)
    (`self.TakeHit` Data)))

(event `ServerTakeHit`
  (params (Data :type "/Game/KobWar/LogicComponents/HitReceiverComponent/Struct_TakeHitData Structure"))
  (`self.MulticastTakeHit` Data)
  (if (not (`Pawn.IsLocallyControlled` (`self.Owner`)))
    (`self.TakeHit` Data)))

(event `MulticastTakeHit`
  (params (Data :type "/Game/KobWar/LogicComponents/HitReceiverComponent/Struct_TakeHitData Structure"))
  (if (not (`Pawn.IsLocallyControlled` (`self.Owner`)))
    (`self.TakeHit` Data)))

(event `LocalSetActorRot`
  (params (NewYaw :type "Float (double-precision)"))
  (if (`Pawn.IsLocallyControlled` (`self.Owner`))
    (`self.ServerSetActorRot` NewYaw)
    (`self.SetActorRot` NewYaw)))

(event `ServerSetActorRot`
  (params (NewYaw :type "Float (double-precision)"))
  (`self.MulticastSetActorRot` NewYaw)
  (`self.SetActorRot` NewYaw))

(event `MulticastSetActorRot`
  (params (NewYaw :type "Float (double-precision)"))
  (if (not (`Pawn.IsLocallyControlled` (`self.Owner`)))
    (`self.SetActorRot` NewYaw)))

(fn `InitOwner`
  (bind _asbp_player_character_base (cast `/Game/KobWar/BP_PlayerCharacterBase` (`self.GetOwner`)))
  (set `self.Owner` _asbp_player_character_base))

(fn `SetActorRot`
  (params (Yaw :type "Float (double-precision)"))
  (`Actor.K2_SetActorRotation` (`self.Owner`) (`KismetMathLibrary.MakeRotator` 0.0 0.0 Yaw) false))

(fn `TakeHit`
  (params (Data :type "/Game/KobWar/LogicComponents/HitReceiverComponent/Struct_TakeHitData Structure"))
  (locals (TakeHitData :type "/Game/KobWar/LogicComponents/HitReceiverComponent/Struct_TakeHitData Structure"))
  (bind _owner (`self.Owner`))
  (bind ((`Attacker_2_86A4A7BB41F2A8C6B1FB968758C1ABC1` _attacker) (`IsDodged_19_D6A768B548C52E6EBCD3E892790EE0CA` _isdodged)) (break `/Game/KobWar/LogicComponents/HitReceiverComponent/Struct_TakeHitData` (`local.TakeHitData`)))
  (if (`Pawn.IsLocallyControlled` _owner)
    (set `local.TakeHitData` Data)
    (`|ExecutionSequence`
      (:`then_0`
        (if (not _isdodged)
          (`self.LocalSetActorRot` (.yaw (`KismetMathLibrary.FindLookAtRotation` (`Actor.K2_GetActorLocation` _owner) (`Actor.K2_GetActorLocation` _attacker))))
          (`ActionControlComponent.ForceActivateStagger` (`KobWarCharacter.ActionControl` _owner)))))))