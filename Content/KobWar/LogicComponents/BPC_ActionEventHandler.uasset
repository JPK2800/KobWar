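; Player character component that handles named action events to turn the character during actions, toward the lock-on target or camera-relative movement input.
; On possession the local client has the server set Owner, whose OnRep binds to ActionControl's fire-action event.
; HandleEvents splits "Name|Params" strings into snap or interpolated turns, the latter via BPC_InterpToDir.
; Turns apply locally first, then replicate through server and multicast events that skip the controlling client.
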(event `self.ReceiveBeginPlay`
  (bind _asbp_player_character_base (cast `/Game/KobWar/BP_PlayerCharacterBase` (`self.GetOwner`)))
  (add `KobWarCharacter.OnPlayerPossession` _asbp_player_character_base (delegate `OnPossessed`)))

(event `OnPossessed`
  (params (PlayerController :type "PlayerController Object Reference"))
  (`self.InitOwner`))

(event `ServerSetOwner`
  (params (NewOwner :type "/Game/KobWar/BP_PlayerCharacterBase Object Reference"))
  (set `self.Owner` NewOwner))

(event `LocalAddInterpDirComponent`
  (params (TurnSpeed :type "Float (double-precision)") (TargetRotation :type "Rotator Structure"))
  (bind _owner (`self.Owner`))
  (`|AddComponentByClass` _owner "/Game/KobWar/LogicComponents/EventComponent/BPC_InterpToDir.BPC_InterpToDir_C" _owner TurnSpeed TargetRotation))

(event `ServerAddInterpToInputDirComponent`
  (params (TurnSpeed :type "Float (double-precision)") (TargetRotation :type "Rotator Structure"))
  (`self.MulticastAddInterpToInputDirComponent` TurnSpeed TargetRotation))

(event `MulticastAddInterpToInputDirComponent`
  (params (TurnSpeed :type "Float (double-precision)") (TargetRotation :type "Rotator Structure"))
  (bind _owner (`self.Owner`))
  (`/Engine/EditorBlueprintResources/StandardMacros.IsValid` _owner
    (:`Is Valid`
      (if (not (`Pawn.IsLocallyControlled` _owner))
        (`self.LocalAddInterpDirComponent` TurnSpeed TargetRotation)))))

(event `LocalSnapToInputRot`
  (params (TargetRotation :type "Rotator Structure"))
  (`Actor.K2_SetActorRotation` (`self.Owner`) TargetRotation false))

(event `ServerSnapToInputRot`
  (params (TargetRotation :type "Rotator Structure"))
  (`self.MulticastSnapToInputRot` TargetRotation))

(event `MulticastSnapToInputRot`
  (params (TargetRotation :type "Rotator Structure"))
  (bind _owner (`self.Owner`))
  (`/Engine/EditorBlueprintResources/StandardMacros.IsValid` _owner
    (:`Is Valid`
      (if (not (`Pawn.IsLocallyControlled` _owner))
        (`self.LocalSnapToInputRot` TargetRotation)))))

(fn `EventInterpToInputDir`
  (params (ParamData :type String))
  (locals (TurnRate :type "Float (double-precision)" :default 25.0) (AdditionalYaw :type "Float (double-precision)") (ForceInputDir :type Boolean))
  (bind _owner (`self.Owner`))
  (bind _turnrate (`local.TurnRate`))
  (bind _turnrate_2 (`local.TurnRate`))
  (bind _cameraboom (`KobWarCharacter.CameraBoom` _owner))
  (`|ExecutionSequence`
    (:`then_0`
      (if (not (`KismetStringLibrary.IsEmpty` ParamData))
        (switch `string` ParamData
          (:`UseInputDir`
            (set `local.ForceInputDir` true)))))
    (:`then_1`
      (`/Engine/EditorBlueprintResources/StandardMacros.IsValid` _owner
        (:`Is Valid`
          (if (`Pawn.IsLocallyControlled` _owner)
            (if (`local.ForceInputDir`)
              (bind _returnvalue (`KobWarCharacter.GetCurrentMovementInput` _owner :!label _label))
              (`/Engine/EditorBlueprintResources/StandardMacros.IsValid` _cameraboom
                (:`Is Valid`
                  (bind (_x _y) (`KismetMathLibrary.BreakVector2D` _returnvalue))
                  (if (> _y 0.05)
                    (bind _returnvalue_2 (`KismetMathLibrary.MakeRotator` (.roll (`SpringArmComponent.GetTargetRotation` _cameraboom)) 0.0 (+ (.yaw (`SpringArmComponent.GetTargetRotation` _cameraboom)) _x (`local.AdditionalYaw`))))
                    (`self.LocalAddInterpDirComponent` _turnrate_2 _returnvalue_2)
                    (`self.ServerAddInterpToInputDirComponent` _turnrate_2 _returnvalue_2))))
              (else
                (bind (_targetcomponent _returnvalue_3) (`LockOnComponent.GetCurrentLockOnTarget` (`/Game/KobWar/BP_PlayerCharacterBase.BPC_LockOnControl` _owner)))
                (if _returnvalue_3
                  (bind _returnvalue_4 (`KismetMathLibrary.MakeRotator` 0.0 0.0 (.yaw (`KismetMathLibrary.FindLookAtRotation` (`SceneComponent.K2_GetComponentLocation` (`KobWarCharacter.LockOnTargetComponent` (`self.Owner`))) (`SceneComponent.K2_GetComponentLocation` _targetcomponent)))))
                  (`self.LocalAddInterpDirComponent` _turnrate _returnvalue_4)
                  (`self.ServerAddInterpToInputDirComponent` _turnrate _returnvalue_4)
                  (else
                    (goto _label)))))))))))

(fn `EventSnapToInputDir`
  (params (ParamData :type String))
  (locals (ForceInputDir :type Boolean))
  (bind _owner (`self.Owner`))
  (bind _cameraboom (`KobWarCharacter.CameraBoom` _owner))
  (`|ExecutionSequence`
    (:`then_0`
      (if (not (`KismetStringLibrary.IsEmpty` ParamData))
        (switch `string` ParamData
          (:`UseInputDir`
            (set `local.ForceInputDir` true)))))
    (:`then_1`
      (`/Engine/EditorBlueprintResources/StandardMacros.IsValid` _owner
        (:`Is Valid`
          (if (`Pawn.IsLocallyControlled` _owner)
            (if (`local.ForceInputDir`)
              (bind _returnvalue (`KobWarCharacter.GetCurrentMovementInput` _owner :!label _label))
              (`/Engine/EditorBlueprintResources/StandardMacros.IsValid` _cameraboom
                (:`Is Valid`
                  (bind (_x _y) (`KismetMathLibrary.BreakVector2D` _returnvalue))
                  (if (> _y 0.4)
                    (bind _returnvalue_2 (`KismetMathLibrary.MakeRotator` (.roll (`SpringArmComponent.GetTargetRotation` _cameraboom)) 0.0 (+ (.yaw (`SpringArmComponent.GetTargetRotation` _cameraboom)) _x)))
                    (`self.LocalSnapToInputRot` _returnvalue_2)
                    (`self.ServerSnapToInputRot` _returnvalue_2))))
              (else
                (bind (_targetcomponent _returnvalue_3) (`LockOnComponent.GetCurrentLockOnTarget` (`/Game/KobWar/BP_PlayerCharacterBase.BPC_LockOnControl` _owner)))
                (if _returnvalue_3
                  (bind _returnvalue_4 (`KismetMathLibrary.MakeRotator` 0.0 0.0 (.yaw (`KismetMathLibrary.FindLookAtRotation` (`SceneComponent.K2_GetComponentLocation` (`KobWarCharacter.LockOnTargetComponent` (`self.Owner`))) (`SceneComponent.K2_GetComponentLocation` _targetcomponent)))))
                  (`self.LocalSnapToInputRot` _returnvalue_4)
                  (`self.ServerSnapToInputRot` _returnvalue_4)
                  (else
                    (goto _label)))))))))))

(fn `HandleEvents`
  (params (Event :type String))
  (locals (EventName :type String) (EventParams :type String))
  (bind (_lefts _rights _returnvalue) (`KismetStringLibrary.Split` Event "|"))
  (if _returnvalue
    (set `local.EventName` _lefts)
    (set `local.EventParams` _rights)
    (else
      (set `local.EventName` Event)))
  (switch `string` (`local.EventName`)
    (:`Default`
      (`KismetSystemLibrary.PrintString` (`KismetStringLibrary.Concat_StrStr` Event " is an unknown action event!")))
    (:`SnapToInputDir`
      (`self.EventSnapToInputDir` (`local.EventParams`)))
    (:`InterpToInputDir`
      (`self.EventInterpToInputDir` (`local.EventParams`)))))

(fn `InitOwner`
  (bind _asbp_player_character_base (cast `/Game/KobWar/BP_PlayerCharacterBase` (`self.GetOwner`)))
  (if (`Pawn.IsLocallyControlled` _asbp_player_character_base)
    (`self.ServerSetOwner` _asbp_player_character_base)))

(fn `OnRep_Owner`
  (bind _owner (`self.Owner`))
  (bind _actioncontrol (`KobWarCharacter.ActionControl` _owner))
  (`/Engine/EditorBlueprintResources/StandardMacros.IsValid` _owner
    (:`Is Valid`
      (if (`Pawn.IsLocallyControlled` _owner)
        (`/Engine/EditorBlueprintResources/StandardMacros.IsValid` _actioncontrol
          (:`Is Valid`
            (bind _output_get (set `self.LocalActionControl` _actioncontrol))
            (add `ActionControlComponent.OnFireActionEvent` _output_get (`|CreateDelegate` :!event `HandleEvents`))))))))

(fn `UpdateMoveDir`
  (params (Direction :type "Vector2D Structure") (Value :type "Float (double-precision)"))
  (set `self.MovementDir` Direction)
  (set `self.MovementMagnitude` Value))