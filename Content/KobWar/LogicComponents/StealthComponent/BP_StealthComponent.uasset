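; Stealth component for a player character that cloaks the owner with distortion materials and restores the originals when stealth ends.
; Stealth changes set the flag locally and send it through a server event, with a RepNotify refreshing materials via the appearance and equipment components.
; Leaving stealth spawns a team-colored poof ring.
; A hit-receiver binding forwards damage taken to the component's owner-damage handler.
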(event `self.ReceiveBeginPlay`
  (bind _isstealthed (`self.IsStealthed`))
  (bind _asbp_player_character_base (cast `/Game/KobWar/BP_PlayerCharacterBase` (`self.GetOwner`)))
  (set `self.GameOwner` _asbp_player_character_base)
  (if _isstealthed
    (`self.OnStealthChange` _isstealthed))
  (add `self.OnStealthStateChange` (`|CreateDelegate` :!event `OnStealthChange`))
  (add `self.OnStealthStateChange` (`|CreateDelegate` :!event `OnStealthChange`)))

(event `self.BindToTakeHit`
  (bind _gameowner (`self.GameOwner`))
  (`/Engine/EditorBlueprintResources/StandardMacros.IsValid` _gameowner
    (:`Is Valid`
      (add `/Game/KobWar/LogicComponents/HitReceiverComponent/BPC_HitReceiverComponent.OnTakeHit` (`/Game/KobWar/BP_PlayerCharacterBase.BPC_HitReceiverComponent` _gameowner) (`|CreateDelegate` :!event `TakeHitEvent`)))))

(event `ServerSetStealthed`
  (params (Stealth :type Boolean))
  (if (not (`Pawn.IsLocallyControlled` (`self.GameOwner`)))
    (set `self.IsStealthed` Stealth)
    (`self.OnStealthUpdateMats` Stealth)))

(fn `OnRep_IsStealthed`
  (`self.OnStealthUpdateMats` (`self.IsStealthed`)))

(fn `OnStealthChange`
  (params (Toggle :type Boolean))
  (set `self.IsStealthed` Toggle)
  (`self.ServerSetStealthed` Toggle))

(fn `OnStealthUpdateMats`
  (params (Toggle :type Boolean))
  (bind _gameowner (`self.GameOwner`))
  (bind _returnvalue (`Actor.GetComponentByClass` _gameowner "/Game/KobWar/LogicComponents/Equipment/BPC_EquipmentHandler.BPC_EquipmentHandler_C"))
  (bind _bpc_appearancecontrol (`/Game/KobWar/BP_PlayerCharacterBase.BPC_AppearanceControl` _gameowner))
  (`/Engine/EditorBlueprintResources/StandardMacros.IsValid` _gameowner
    (:`Is Valid`
      (`|ExecutionSequence`
        (:`then_0`
          (`/Engine/EditorBlueprintResources/StandardMacros.IsValid` _bpc_appearancecontrol
            (:`Is Valid`
              (if Toggle
                (`/Game/KobWar/LogicComponents/Appearance/BPC_AppearanceControl.ApplyMaterialToAll` _bpc_appearancecontrol "/Game/KobWar/LogicComponents/StealthComponent/MI_DistortStealth.MI_DistortStealth" "/Game/KobWar/LogicComponents/StealthComponent/MI_DistortStealthSmall.MI_DistortStealthSmall" "/Game/KobWar/LogicComponents/StealthComponent/MI_DistortStealthSmall.MI_DistortStealthSmall" "/Game/KobWar/LogicComponents/StealthComponent/MI_DistortStealth.MI_DistortStealth")
                (else
                  (`/Game/KobWar/LogicComponents/Appearance/BPC_AppearanceControl.ReapplyMaterials` _bpc_appearancecontrol))))))
        (:`then_1`
          (`/Engine/EditorBlueprintResources/StandardMacros.IsValid` _returnvalue
            (:`Is Valid`
              (if Toggle
                (`/Game/KobWar/LogicComponents/Equipment/BPC_EquipmentHandler.ApplyMaterialToAll` _returnvalue "/Game/KobWar/LogicComponents/StealthComponent/MI_DistortStealth.MI_DistortStealth" "/Game/KobWar/LogicComponents/StealthComponent/MI_DistortStealth.MI_DistortStealth")
                (else
                  (`/Game/KobWar/LogicComponents/Equipment/BPC_EquipmentHandler.ReapplyMaterials` _returnvalue)))
              (if (not (`self.IsStealthed`))
                (`self.SpawnEndStealthEffect`)))))))))

(fn `SpawnEndStealthEffect`
  (bind _gameowner (`self.GameOwner`))
  (bind _returnvalue (`NiagaraFunctionLibrary.SpawnSystemAtLocation` "/Game/KobWar/Effects/P_PoofRing.P_PoofRing" (`Actor.K2_GetActorLocation` _gameowner)))
  (bind _returnvalue_2 (`KobWarCharacter.GetCharacterTeamId` _gameowner))
  (if (== _returnvalue_2 1)
    (`FXSystemComponent.SetColorParameter` _returnvalue "ColorEnd" (struct :`G` 0.048248 :`B` 0.302083 :`A` 1.0))
    (`FXSystemComponent.SetColorParameter` _returnvalue "ColorBegin" (struct :`G` 0.844235 :`B` 0.947917 :`A` 1.0))
    (elif (== _returnvalue_2 2)
      (`FXSystemComponent.SetColorParameter` _returnvalue "ColorEnd" (struct :`R` 0.244792 :`B` 0.243436 :`A` 1.0))
      (`FXSystemComponent.SetColorParameter` _returnvalue "ColorBegin" (struct :`R` 0.947917 :`G` 0.057526 :`A` 1.0))
      (else
        (`FXSystemComponent.SetColorParameter` _returnvalue "ColorEnd" (struct :`R` 0.180156 :`G` 0.17045 :`B` 0.244792 :`A` 1.0))
        (`FXSystemComponent.SetColorParameter` _returnvalue "ColorBegin" (struct :`R` 0.897569 :`G` 0.947917 :`B` 0.938426 :`A` 1.0))))))

(fn `TakeHitEvent`
  (params (Damage :type Integer))
  (`self.OnOwnerDamageTaken` (`KismetMathLibrary.Conv_IntToDouble` Damage)))