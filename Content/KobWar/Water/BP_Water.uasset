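; BP_Water is a water actor that spawns ring effects at the surface under characters inside it.
; Box overlap events maintain a map of characters to their last known locations.
; Each tick, a moved character spawns P_WaterRings at plane height and updates its location.
; Stationary characters flip a shared AlternateTick flag, spawning P_WaterRingsSmall on every other flip.
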(event `self.ReceiveTick`
  (params (DeltaSeconds :type "Float (single-precision)"))
  (`self.SpawnRingsOnOverlappingChars`))

(event `self.Box.OnComponentBeginOverlap`
  (params (OverlappedComponent :type "PrimitiveComponent Object Reference") (OtherActor :type "Actor Object Reference") (OtherComp :type "PrimitiveComponent Object Reference") (OtherBodyIndex :type Integer) (bFromSweep :type Boolean) (SweepResult :type "HitResult Structure (by ref)"))
  (bind _ascharacter (cast `Character` OtherActor))
  (`BlueprintMapLibrary.Map_Add` (`self.OverlappedCharacters`) _ascharacter (`self.K2_GetActorLocation` _ascharacter)))

(event `self.Box.OnComponentEndOverlap`
  (params (OverlappedComponent :type "PrimitiveComponent Object Reference") (OtherActor :type "Actor Object Reference") (OtherComp :type "PrimitiveComponent Object Reference") (OtherBodyIndex :type Integer))
  (bind _overlappedcharacters (`self.OverlappedCharacters`))
  (bind _ascharacter (cast `Character` OtherActor))
  (if (`BlueprintMapLibrary.Map_Contains` _overlappedcharacters _ascharacter)
    (`BlueprintMapLibrary.Map_Remove` _overlappedcharacters _ascharacter)))

(fn `SpawnRingsOnOverlappingChars`
  (locals (CharsToRemove :type "Array of Character Object Reference"))
  (bind _overlappedcharacters (`self.OverlappedCharacters`))
  (bind (_returnvalue_x _returnvalue_y _returnvalue_z) (`KismetMathLibrary.BreakVector` (`SceneComponent.K2_GetComponentLocation` (`self.Plane`))))
  (bind _returnvalue (+ _returnvalue_z 1.0))
  (bind _keys (`BlueprintMapLibrary.Map_Keys` _overlappedcharacters))
  (for _array_element _keys
    (`/Engine/EditorBlueprintResources/StandardMacros.IsValid` _array_element
      (:`Is Valid`
        (bind (_value _returnvalue_2) (`BlueprintMapLibrary.Map_Find` _overlappedcharacters _array_element))
        (if _returnvalue_2
          (bind _returnvalue_3 (`self.K2_GetActorLocation` _array_element))
          (if (`KismetMathLibrary.NotEqualExactly_VectorVector` _returnvalue_3 _value)
            (`BlueprintMapLibrary.Map_Add` _overlappedcharacters _array_element _returnvalue_3)
            (bind (_returnvalue_x_2 _returnvalue_y_2) (`KismetMathLibrary.BreakVector` (`self.K2_GetActorLocation` _array_element)))
            (`NiagaraFunctionLibrary.SpawnSystemAtLocation` "/Game/KobWar/Effects/P_WaterRings.P_WaterRings" (`KismetMathLibrary.MakeVector` _returnvalue_x_2 _returnvalue_y_2 _returnvalue))
            (else
              (set `self.bAlternateTick` (not (`self.bAlternateTick`)))
              (if (`self.bAlternateTick`)
                (`NiagaraFunctionLibrary.SpawnSystemAtLocation` "/Game/KobWar/Effects/P_WaterRingsSmall.P_WaterRingsSmall" (`KismetMathLibrary.MakeVector` _returnvalue_x_2 _returnvalue_y_2 _returnvalue)))))))
      (:`Is Not Valid`
        (`KismetArrayLibrary.Array_Add` (`local.CharsToRemove`)))))
  (for _array_element_2 (`local.CharsToRemove`)
    (`BlueprintMapLibrary.Map_Remove` (`self.OverlappedCharacters`) _array_element_2)))

(fn `UserConstructionScript`)