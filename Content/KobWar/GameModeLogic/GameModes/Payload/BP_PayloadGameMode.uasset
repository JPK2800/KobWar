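; Payload game mode that tracks cart attackers and defenders and feeds match progress into BP_PayloadGameState.
; InitGameState loads payload data into that state and caches it for writing cart distance, checkpoints and next-round team updates.
; Add and remove functions maintain pusher and defender lists.
; A looping one-second authority timer prunes invalid entries and calls an occupancy update only when either count changes.
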(event `self.ReceiveBeginPlay`
  (`parent.ReceiveBeginPlay`)
  (if (`self.HasAuthority`)
    (`KismetSystemLibrary.K2_SetTimerDelegate` (delegate `CartValidationEvent`) 1.0 true)))

(event `CartValidationEvent`
  (bind (_attackersoncart _defendersoncart) (`self.ValidateEachCartUnit`))
  (if (or (!= (`self.AttackersOnCart`) _attackersoncart) (!= (`self.DefendersOnCart`) _defendersoncart))
    (bind _output_get (set `self.AttackersOnCart` _attackersoncart))
    (bind _output_get_2 (set `self.DefendersOnCart` _defendersoncart))
    (`self.UpdateOccupancy` _output_get _output_get_2)))

(fn `AddCartDefender`
  (params (Character :type "/Game/KobWar/BP_PlayerCharacterBase Object Reference"))
  (`KismetArrayLibrary.Array_AddUnique` (`self.CartDefenders`) Character))

(fn `AddCartPusher`
  (params (Character :type "/Game/KobWar/BP_PlayerCharacterBase Object Reference"))
  (`KismetArrayLibrary.Array_AddUnique` (`self.CartPushers`) Character))

(fn `InitGameState`
  (`parent.InitGameState`)
  (bind _asbp_payload_game_state (cast `/Game/KobWar/GameModeLogic/GameModes/Payload/BP_PayloadGameState` (`self.BPGameState`)))
  (`/Game/KobWar/GameModeLogic/GameModes/Payload/BP_PayloadGameState.LoadPayloadGameModeData` _asbp_payload_game_state (`self.PayloadData`))
  (set `self.SpecificGameState` _asbp_payload_game_state))

(fn `RemoveCartDefender`
  (params (Character :type "/Game/KobWar/BP_PlayerCharacterBase Object Reference"))
  (`KismetArrayLibrary.Array_RemoveItem` (`self.CartDefenders`) Character))

(fn `RemoveCartPusher`
  (params (Character :type "/Game/KobWar/BP_PlayerCharacterBase Object Reference"))
  (`KismetArrayLibrary.Array_RemoveItem` (`self.CartPushers`) Character))

(fn `UpdateCartDistancePercent`
  (params (CartDistancePercent :type "Float (double-precision)"))
  (bind _specificgamestate (`self.SpecificGameState`))
  (`/Engine/EditorBlueprintResources/StandardMacros.IsValid` _specificgamestate
    (:`Is Valid`
      (bind _structout (setmembers `/Game/KobWar/GameModeLogic/GameModes/Payload/Struct_PayloadModeProgress` :`StructRef` (`|Copy` (`/Game/KobWar/GameModeLogic/GameModes/Payload/BP_PayloadGameState.PayloadProgress` _specificgamestate)) :`PayloadProgressPercent` CartDistancePercent))
      (set `/Game/KobWar/GameModeLogic/GameModes/Payload/BP_PayloadGameState.PayloadProgress` _structout _specificgamestate))))

(fn `UpdateCheckpointData`
  (params (CheckpointDistances :type "Map of Byte to Float (double-precision)") (TotalSplineDistance :type "Float (double-precision)"))
  (bind _specificgamestate (`self.SpecificGameState`))
  (`/Engine/EditorBlueprintResources/StandardMacros.IsValid` _specificgamestate
    (:`Is Valid`
      (`/Game/KobWar/GameModeLogic/GameModes/Payload/BP_PayloadGameState.UpdatePayloadCheckpointData` _specificgamestate CheckpointDistances TotalSplineDistance))))

(fn `UpdateCheckpointReached`
  (params (Checkpoint :type Byte))
  (bind _specificgamestate (`self.SpecificGameState`))
  (`/Engine/EditorBlueprintResources/StandardMacros.IsValid` _specificgamestate
    (:`Is Valid`
      (bind _structout (setmembers `/Game/KobWar/GameModeLogic/GameModes/Payload/Struct_PayloadModeProgress` :`StructRef` (`|Copy` (`/Game/KobWar/GameModeLogic/GameModes/Payload/BP_PayloadGameState.PayloadProgress` _specificgamestate)) :`CurrentRoundCapturedPoints` Checkpoint))
      (set `/Game/KobWar/GameModeLogic/GameModes/Payload/BP_PayloadGameState.PayloadProgress` _structout _specificgamestate))))

(fn `UpdateRoundEnd`
  (params (RoundCompleted :type Byte))
  (if (< RoundCompleted (`self.RoundCount`))
    (`/Game/KobWar/GameModeLogic/GameModes/Payload/BP_PayloadGameState.UpdatePlayerTeamForRound` (`self.SpecificGameState`) (+ RoundCompleted 1))))

(fn `UserConstructionScript`
  (`parent.UserConstructionScript`))

(fn `ValidateEachCartUnit`
  (returns (AttackersOnCart :type Byte) (DefendersOnCart :type Byte))
  (locals (NewCartPushers :type "Array of /Game/KobWar/BP_PlayerCharacterBase Object Reference") (NewCartDefenders :type "Array of /Game/KobWar/BP_PlayerCharacterBase Object Reference"))
  (`|ExecutionSequence`
    (:`then_0`
      (for _array_element (`self.CartPushers`)
        (`/Engine/EditorBlueprintResources/StandardMacros.IsValid` _array_element
          (:`Is Valid`
            (`KismetArrayLibrary.Array_Add` (`local.NewCartPushers`) _array_element))))
      (set `self.CartPushers` (`local.NewCartPushers`)))
    (:`then_1`
      (for _array_element_2 (`self.CartDefenders`)
        (`/Engine/EditorBlueprintResources/StandardMacros.IsValid` _array_element_2
          (:`Is Valid`
            (`KismetArrayLibrary.Array_Add` (`local.NewCartDefenders`) _array_element_2))))
      (set `self.CartDefenders` (`local.NewCartDefenders`)))
    (:`then_2`
      (return (`KismetMathLibrary.Conv_IntToByte` (`KismetArrayLibrary.Array_Length` (`self.CartPushers`))) (`KismetMathLibrary.Conv_IntToByte` (`KismetArrayLibrary.Array_Length` (`self.CartDefenders`)))))))