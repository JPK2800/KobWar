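; Server-authoritative payload cart for Payload mode that attackers escort along a spline.
; Box overlaps register players with BP_PayloadGameMode as pushers or defenders by team; its occupancy callback stops the cart when contested or empty, otherwise scaling speed up to four pushers.
; Tick advances spline distance, reporting throttled progress and checkpoints, which are placed actors projected onto the spline.
; Clients disable the box and follow the cart through CartTf's RepNotify.
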(event `self.ReceiveBeginPlay`
  (if (`self.HasAuthority`)
    (`self.BindToGameMode`)
    (`self.InitCheckpoints`)
    (`self.K2_SetActorLocation` (`SplineComponent.GetLocationAtSplinePoint` (`self.Spline`) 0 "World"))
    (else
      (`PrimitiveComponent.SetCollisionEnabled` (`self.Box`) "NoCollision"))))

(event `self.ReceiveTick`
  (params (DeltaSeconds :type "Float (single-precision)"))
  (`self.MoveAlongSplineStep` DeltaSeconds))

(event `self.Box.OnComponentBeginOverlap`
  (params (OverlappedComponent :type "PrimitiveComponent Object Reference") (OtherActor :type "Actor Object Reference") (OtherComp :type "PrimitiveComponent Object Reference") (OtherBodyIndex :type Integer) (bFromSweep :type Boolean) (SweepResult :type "HitResult Structure (by ref)"))
  (bind _payloadgamemode (`self.PayloadGameMode`))
  (if (`self.HasAuthority`)
    (bind _asbp_player_character_base (cast `/Game/KobWar/BP_PlayerCharacterBase` OtherActor))
    (bind _returnvalue (`KobWarCharacter.GetCharacterTeamId` _asbp_player_character_base))
    (bind _asbp_payload_game_state (cast `/Game/KobWar/GameModeLogic/GameModes/Payload/BP_PayloadGameState` (`GameplayStatics.GetGameState`)))
    (bind (_payloaddata_isblackattacking _payloaddata_iswhiteattacking) (break `/Game/KobWar/GameModeLogic/GameModes/Payload/Struct_PayloadModeData` (`/Game/KobWar/GameModeLogic/GameModes/Payload/BP_PayloadGameState.PayloadData` _asbp_payload_game_state)))
    (if (or (and (== _returnvalue (enumliteral `ETeam` "Team_1")) _payloaddata_iswhiteattacking) (and (== _returnvalue (enumliteral `ETeam` "Team_2")) _payloaddata_isblackattacking))
      (`/Engine/EditorBlueprintResources/StandardMacros.IsValid` _payloadgamemode
        (:`Is Valid`
          (`/Game/KobWar/GameModeLogic/GameModes/Payload/BP_PayloadGameMode.AddCartPusher` _payloadgamemode _asbp_player_character_base)))
      (elif (or (and (== _returnvalue (enumliteral `ETeam` "Team_1")) _payloaddata_isblackattacking) (and (== _returnvalue (enumliteral `ETeam` "Team_2")) _payloaddata_iswhiteattacking))
        (`/Engine/EditorBlueprintResources/StandardMacros.IsValid` _payloadgamemode
          (:`Is Valid`
            (`/Game/KobWar/GameModeLogic/GameModes/Payload/BP_PayloadGameMode.AddCartDefender` _payloadgamemode _asbp_player_character_base)))))))

(event `self.Box.OnComponentEndOverlap`
  (params (OverlappedComponent :type "PrimitiveComponent Object Reference") (OtherActor :type "Actor Object Reference") (OtherComp :type "PrimitiveComponent Object Reference") (OtherBodyIndex :type Integer))
  (bind _payloadgamemode (`self.PayloadGameMode`))
  (if (`self.HasAuthority`)
    (bind _asbp_player_character_base (cast `/Game/KobWar/BP_PlayerCharacterBase` OtherActor))
    (bind _returnvalue (`KobWarCharacter.GetCharacterTeamId` _asbp_player_character_base))
    (bind _asbp_payload_game_state (cast `/Game/KobWar/GameModeLogic/GameModes/Payload/BP_PayloadGameState` (`GameplayStatics.GetGameState`)))
    (bind (_payloaddata_isblackattacking _payloaddata_iswhiteattacking) (break `/Game/KobWar/GameModeLogic/GameModes/Payload/Struct_PayloadModeData` (`/Game/KobWar/GameModeLogic/GameModes/Payload/BP_PayloadGameState.PayloadData` _asbp_payload_game_state)))
    (if (or (and (== _returnvalue (enumliteral `ETeam` "Team_1")) _payloaddata_iswhiteattacking) (and (== _returnvalue (enumliteral `ETeam` "Team_2")) _payloaddata_isblackattacking))
      (`/Engine/EditorBlueprintResources/StandardMacros.IsValid` _payloadgamemode
        (:`Is Valid`
          (`/Game/KobWar/GameModeLogic/GameModes/Payload/BP_PayloadGameMode.RemoveCartPusher` _payloadgamemode _asbp_player_character_base)))
      (elif (or (and (== _returnvalue (enumliteral `ETeam` "Team_1")) _payloaddata_isblackattacking) (and (== _returnvalue (enumliteral `ETeam` "Team_2")) _payloaddata_iswhiteattacking))
        (`/Engine/EditorBlueprintResources/StandardMacros.IsValid` _payloadgamemode
          (:`Is Valid`
            (`/Game/KobWar/GameModeLogic/GameModes/Payload/BP_PayloadGameMode.RemoveCartDefender` _payloadgamemode _asbp_player_character_base)))))))

(fn `BindToGameMode`
  (bind _asbp_payload_game_mode (cast `/Game/KobWar/GameModeLogic/GameModes/Payload/BP_PayloadGameMode` (`GameplayStatics.GetGameMode`)))
  (bind _output_get (set `self.PayloadGameMode` _asbp_payload_game_mode))
  (add `/Game/KobWar/GameModeLogic/GameModes/Payload/BP_PayloadGameMode.UpdateOccupancy` _output_get (`|CreateDelegate` :!event `UpdateOccupancyFromGameMode`)))

(fn `InitCheckpoints`
  (bind _spline (`self.Spline`))
  (bind _payloadgamemode (`self.PayloadGameMode`))
  (if (`self.HasAuthority`)
    (bind _outactors (`GameplayStatics.GetAllActorsOfClass` "/Game/KobWar/GameModeLogic/GameModes/Payload/PayloadActor/BP_PayloadCheckpoint.BP_PayloadCheckpoint_C"))
    (for _array_element _outactors
      (`BlueprintMapLibrary.Map_Add` (`self.Checkpoints`) (`/Game/KobWar/GameModeLogic/GameModes/Payload/PayloadActor/BP_PayloadCheckpoint.CheckpointNum` _array_element) (`SplineComponent.GetDistanceAlongSplineAtSplineInputKey` _spline (`SplineComponent.FindInputKeyClosestToWorldLocation` _spline (`self.K2_GetActorLocation` _array_element)))))
    (`/Engine/EditorBlueprintResources/StandardMacros.IsValid` _payloadgamemode
      (:`Is Valid`
        (`/Game/KobWar/GameModeLogic/GameModes/Payload/BP_PayloadGameMode.UpdateCheckpointData` _payloadgamemode (`self.Checkpoints`) (`SplineComponent.GetSplineLength` (`self.Spline`)))))))

(fn `MoveAlongSplineStep`
  (params (DeltaTime :type "Float (double-precision)"))
  (bind _spline (`self.Spline`))
  (bind _checkpoints (`self.Checkpoints`))
  (bind _returnvalue (`KismetMathLibrary.Conv_IntToDouble` (`KismetMathLibrary.FFloor` (/ (`self.CurrentDistance`) 32.0))))
  (if (`self.HasAuthority`)
    (if (`self.IsMoving`)
      (`|ExecutionSequence`
        (:`then_0`
          (bind _output_get (set `self.CurrentDistance` (+ (`self.CurrentDistance`) (/ (* (`KismetMathLibrary.MapRangeClamped` (`KismetMathLibrary.Conv_ByteToDouble` (`self.MovePower`)) 0.0 4.0 1000.0 3000.0) DeltaTime) 60.0))))
          (bind _returnvalue_location (`KismetMathLibrary.BreakTransform` (`SplineComponent.GetTransformAtDistanceAlongSpline` _spline _output_get "World" false)))
          (bind _returnvalue_2 (`KismetMathLibrary.Conv_VectorToTransform` _returnvalue_location))
          (`self.K2_SetActorTransform` _returnvalue_2)
          (set `self.CartTf` _returnvalue_2)
          (if (!= _returnvalue (`self.LastReportedDist`))
            (`self.UpdateGameModeProgress` (/ _output_get (`SplineComponent.GetSplineLength` _spline)))
            (set `self.LastReportedDist` _returnvalue)))
        (:`then_1`
          (bind _keys (`BlueprintMapLibrary.Map_Keys` _checkpoints))
          (for _array_element _keys
            (if (> _array_element (`self.CheckpointsReached`))
              (bind (_value _returnvalue_3) (`BlueprintMapLibrary.Map_Find` _checkpoints _array_element))
              (if _returnvalue_3
                (if (>= (`self.CurrentDistance`) _value)
                  (if (< (`self.CheckpointsReached`) _array_element)
                    (bind _output_get_2 (set `self.CheckpointsReached` _array_element))
                    (`self.UpdateGameModePoints` _output_get_2)))))))))))

(fn `MoveCart`
  (params (Magnitude :type Byte))
  (set `self.IsMoving` true)
  (set `self.MovePower` Magnitude))

(fn `OnRep_CartTf`
  (`self.K2_SetActorTransform` (`self.CartTf`)))

(fn `StopCart`
  (set `self.IsMoving` false)
  (set `self.MovePower` 0))

(fn `UpdateGameModePoints`
  (params (AttackerPoints :type Byte))
  (bind _payloadgamemode (`self.PayloadGameMode`))
  (`/Engine/EditorBlueprintResources/StandardMacros.IsValid` _payloadgamemode
    (:`Is Valid`
      (`/Game/KobWar/GameModeLogic/GameModes/Payload/BP_PayloadGameMode.UpdateCheckpointReached` _payloadgamemode AttackerPoints))))

(fn `UpdateGameModeProgress`
  (params (DistancePercent :type "Float (double-precision)"))
  (bind _payloadgamemode (`self.PayloadGameMode`))
  (`/Engine/EditorBlueprintResources/StandardMacros.IsValid` _payloadgamemode
    (:`Is Valid`
      (`/Game/KobWar/GameModeLogic/GameModes/Payload/BP_PayloadGameMode.UpdateCartDistancePercent` _payloadgamemode DistancePercent))))

(fn `UpdateOccupancyFromGameMode`
  (params (AttackesOnCart :type Byte) (DefendersOnCart :type Byte))
  (bind _characterpushcount (`self.CharacterPushCount`))
  (set `self.CharacterPushCount` AttackesOnCart)
  (set `self.CharacterDefendCount` DefendersOnCart)
  (if (or (> (`self.CharacterDefendCount`) 0) (== _characterpushcount 0))
    (`self.StopCart`)
    (elif (>= _characterpushcount 4)
      (`self.MoveCart` 4)
      (else
        (`self.MoveCart` _characterpushcount)))))

(fn `UserConstructionScript`)