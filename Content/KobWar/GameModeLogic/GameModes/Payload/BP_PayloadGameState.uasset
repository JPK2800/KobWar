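; Game State for the Payload game mode that replicates mode data, payload progress and up to four checkpoint positions.
; Replicated mode data triggers creation of the local progress widget, which OnRep handlers refresh as progress and checkpoints change.
; Checkpoint updates convert spline distances into track fractions relative to current progress.
; Round changes store the round number and, in team modes with side switching, set player teams by round parity.
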(event `LoadPayloadGameModeData`
  (params (PayloadData :type "/Game/KobWar/GameModeLogic/GameModes/Payload/Struct_PayloadModeData Structure"))
  (set `self.PayloadData` PayloadData))

(event `LoadPayloadProgress`
  (params (PayloadProgress :type "/Game/KobWar/GameModeLogic/GameModes/Payload/Struct_PayloadModeProgress Structure"))
  (bind _output_get (set `self.PayloadProgress` PayloadProgress))
  (`self.UpdatePayloadProgress` _output_get))

(fn `CreatePayloadWidget`
  (if (`Controller.IsLocalController` (`GameplayStatics.GetPlayerController` 0))
    (`/Engine/EditorBlueprintResources/StandardMacros.DoOnce` false
      (:`Completed`
        (bind _returnvalue (`|CreateWidget` (`.PayloadProgressWidget_17_1CC1B8A9444B53279CB631B802EFD6FB` (break `/Game/KobWar/GameModeLogic/GameModes/Payload/Struct_PayloadModeData` (`self.PayloadData`))) (`GameplayStatics.GetPlayerController` 0)))
        (bind _aswbp_payload_ui_widget (cast `/Game/KobWar/GameModeLogic/GameModes/Payload/WBP_PayloadUiWidget` _returnvalue))
        (`UserWidget.AddToPlayerScreen` _aswbp_payload_ui_widget 0)
        (set `self.PayloadWidget` _aswbp_payload_ui_widget)))))

(fn `OnRep_Checkpoint1Progress`
  (bind _payloadwidget (`self.PayloadWidget`))
  (`/Engine/EditorBlueprintResources/StandardMacros.IsValid` _payloadwidget
    (:`Is Valid`
      (`/Game/KobWar/GameModeLogic/GameModes/Payload/WBP_PayloadUiWidget.UpdateOneCheckpointPositionData` _payloadwidget (`self.Checkpoint1Progress`)))))

(fn `OnRep_Checkpoint2Progress`
  (bind _payloadwidget (`self.PayloadWidget`))
  (`/Engine/EditorBlueprintResources/StandardMacros.IsValid` _payloadwidget
    (:`Is Valid`
      (`/Game/KobWar/GameModeLogic/GameModes/Payload/WBP_PayloadUiWidget.UpdateOneCheckpointPositionData` _payloadwidget (`self.Checkpoint2Progress`)))))

(fn `OnRep_Checkpoint3Progress`
  (bind _payloadwidget (`self.PayloadWidget`))
  (`/Engine/EditorBlueprintResources/StandardMacros.IsValid` _payloadwidget
    (:`Is Valid`
      (`/Game/KobWar/GameModeLogic/GameModes/Payload/WBP_PayloadUiWidget.UpdateOneCheckpointPositionData` _payloadwidget (`self.Checkpoint3Progress`)))))

(fn `OnRep_Checkpoint4Progress`
  (bind _payloadwidget (`self.PayloadWidget`))
  (`/Engine/EditorBlueprintResources/StandardMacros.IsValid` _payloadwidget
    (:`Is Valid`
      (`/Game/KobWar/GameModeLogic/GameModes/Payload/WBP_PayloadUiWidget.UpdateOneCheckpointPositionData` _payloadwidget (`self.Checkpoint4Progress`)))))

(fn `OnRep_PayloadData`
  (`self.CreatePayloadWidget`))

(fn `OnRep_PayloadProgress`
  (`self.UpdatePayloadProgress` (`self.PayloadProgress`)))

(fn `UpdatePayloadCheckpointData`
  (params (CheckpointDistances :type "Map of Byte to Float (double-precision)") (SplineDistance :type "Float (double-precision)"))
  (bind _payloadprogress_payloadprogresspercent (break `/Game/KobWar/GameModeLogic/GameModes/Payload/Struct_PayloadModeProgress` (`self.PayloadProgress`)))
  (bind _payloadwidget (`self.PayloadWidget`))
  (bind _keys (`BlueprintMapLibrary.Map_Keys` CheckpointDistances))
  (for _array_element _keys
    (switch `int` (`KismetMathLibrary.Conv_ByteToInt` _array_element)
      (:`1`
        (bind _value (`BlueprintMapLibrary.Map_Find` CheckpointDistances _array_element))
        (bind _returnvalue (/ _value SplineDistance))
        (bind _returnvalue_2 (>= _returnvalue _payloadprogress_payloadprogresspercent))
        (bind _output_get (set `self.Checkpoint1Progress` (make `/Game/KobWar/GameModeLogic/GameModes/Payload/Struct_PayloadCapPointProgress` 1 _value _returnvalue _returnvalue_2)))
        (`/Engine/EditorBlueprintResources/StandardMacros.IsValid` (`self.PayloadWidget`)
          (:`Is Valid`
            (`/Game/KobWar/GameModeLogic/GameModes/Payload/WBP_PayloadUiWidget.UpdateOneCheckpointPositionData` _payloadwidget _output_get))))
      (:`2`
        (bind _output_get_2 (set `self.Checkpoint2Progress` (make `/Game/KobWar/GameModeLogic/GameModes/Payload/Struct_PayloadCapPointProgress` 2 _value _returnvalue _returnvalue_2)))
        (`/Engine/EditorBlueprintResources/StandardMacros.IsValid` (`self.PayloadWidget`)
          (:`Is Valid`
            (`/Game/KobWar/GameModeLogic/GameModes/Payload/WBP_PayloadUiWidget.UpdateOneCheckpointPositionData` _payloadwidget _output_get_2))))
      (:`3`
        (bind _output_get_3 (set `self.Checkpoint3Progress` (make `/Game/KobWar/GameModeLogic/GameModes/Payload/Struct_PayloadCapPointProgress` 3 _value _returnvalue _returnvalue_2)))
        (`/Engine/EditorBlueprintResources/StandardMacros.IsValid` (`self.PayloadWidget`)
          (:`Is Valid`
            (`/Game/KobWar/GameModeLogic/GameModes/Payload/WBP_PayloadUiWidget.UpdateOneCheckpointPositionData` _payloadwidget _output_get_3))))
      (:`4`
        (set `self.Checkpoint4Progress` (make `/Game/KobWar/GameModeLogic/GameModes/Payload/Struct_PayloadCapPointProgress` 4 _value _returnvalue _returnvalue_2))
        (`/Engine/EditorBlueprintResources/StandardMacros.IsValid` (`self.PayloadWidget`)
          (:`Is Valid`
            (`/Game/KobWar/GameModeLogic/GameModes/Payload/WBP_PayloadUiWidget.UpdateOneCheckpointPositionData` :`self` _payloadwidget)))))))

(fn `UpdatePayloadProgress`
  (params (PayloadProgress :type "/Game/KobWar/GameModeLogic/GameModes/Payload/Struct_PayloadModeProgress Structure"))
  (bind _payloadwidget (`self.PayloadWidget`))
  (`/Engine/EditorBlueprintResources/StandardMacros.IsValid` _payloadwidget
    (:`Is Valid`
      (`/Game/KobWar/GameModeLogic/GameModes/Payload/WBP_PayloadUiWidget.UpdatePayloadProgress` _payloadwidget PayloadProgress))))

(fn `UpdatePlayerTeamForRound`
  (params (NewRound :type Byte))
  (`|ExecutionSequence`
    (:`then_0`
      (bind _structout (setmembers `/Game/KobWar/GameModeLogic/GameModes/Payload/Struct_PayloadModeProgress` :`StructRef` (`|Copy` (`self.PayloadProgress`)) :`RoundNumber` NewRound))
      (set `self.PayloadProgress` _structout))
    (:`then_1`
      (if (and (`self.IsTeamBased`) (`self.SwitchSideEachRound`))
        (for _array_element (`self.PlayerArray`)
          (bind _asbp_player_state (cast `/Game/KobWar/GameModeLogic/BP_PlayerState` _array_element))
          (bind _internalteam (`/Game/KobWar/GameModeLogic/BP_PlayerState.InternalTeam` _asbp_player_state))
          (if (== _internalteam 1)
            (if (== (mod NewRound 2) 1)
              (`/Game/KobWar/GameModeLogic/BP_PlayerState.SetStateTeam` _asbp_player_state 1)
              (else
                (`/Game/KobWar/GameModeLogic/BP_PlayerState.SetStateTeam` _asbp_player_state 2)))
            (elif (== _internalteam 2)
              (if (== (mod NewRound 2) 1)
                (`/Game/KobWar/GameModeLogic/BP_PlayerState.SetStateTeam` _asbp_player_state 2)
                (else
                  (`/Game/KobWar/GameModeLogic/BP_PlayerState.SetStateTeam` _asbp_player_state 1))))))))))

(fn `UserConstructionScript`
  (`parent.UserConstructionScript`))