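; Payload game mode Blueprint, the BlackAttack variant, which hands its payload configuration to the game state.
; Its InitGameState calls the parent, casts BPGameState to BP_PayloadGameState and loads PayloadData into it through LoadPayloadGameModeData.
; It adds no other logic: BeginPlay and Tick are disabled stubs and construction only calls the parent.
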(fn `InitGameState`
  (`parent.InitGameState`)
  (bind _asbp_payload_game_state (cast `/Game/KobWar/GameModeLogic/GameModes/Payload/BP_PayloadGameState` (`self.BPGameState`)))
  (`/Game/KobWar/GameModeLogic/GameModes/Payload/BP_PayloadGameState.LoadPayloadGameModeData` _asbp_payload_game_state (`self.PayloadData`)))

(fn `UserConstructionScript`
  (`parent.UserConstructionScript`))