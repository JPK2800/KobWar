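; Base game mode for KobWar that handles player connections, team assignment, game start and wave-style respawns.
; On BeginPlay it binds player events and copies its match, team and class rules into BP_GameState.
; SetPlayerTeam checks team caps and the balance ratio, unless imbalanced switching is allowed, before updating the PlayerState.
; Game start initializes the respawn timer, and each respawn trigger resets it, spawns queued controllers and clears the queue.
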(event `self.ReceiveBeginPlay`
  (add `self.OnPlayerConnect` (`|CreateDelegate` :!event `PlayerConnect`))
  (add `self.OnPlayerDisconnect` (`|CreateDelegate` :!event `PlayerDisconnect`))
  (add `self.OnPlayerSetToTeam` (`|CreateDelegate` :!event `PlayerSwitchTeam`))
  (`self.InitGameState`))

(event `self.TriggerRespawnEvent`
  (bind _bpgamestate (`self.BPGameState`))
  (`/Engine/EditorBlueprintResources/StandardMacros.IsValid` _bpgamestate
    (:`Is Valid`
      (`/Game/KobWar/GameModeLogic/BP_GameState.UpdateRespawnTimer` _bpgamestate (+ (`KismetMathLibrary.Now`) (`KismetMathLibrary.MakeTimespan` 0 0 0 (`KismetMathLibrary.FTrunc` (`self.RespawnTime`)))))
      (`self.RespawnQueuedPlayers`)
      (`KismetArrayLibrary.Array_Clear` (`self.RespawnQueue`)))))

(event `self.TriggerGameStartEvent`
  (bind _bpgamestate (`self.BPGameState`))
  (`/Engine/EditorBlueprintResources/StandardMacros.IsValid` _bpgamestate
    (:`Is Valid`
      (`self.InitRespawnTimer`)
      (`/Game/KobWar/GameModeLogic/BP_GameState.UpdateRespawnTimer` _bpgamestate (+ (`KismetMathLibrary.Now`) (`KismetMathLibrary.MakeTimespan` 0 0 0 (`KismetMathLibrary.FTrunc` (`self.RespawnTime`)))))
      (set `/Game/KobWar/GameModeLogic/BP_GameState.GameStarted` true _bpgamestate)
      (`GameplayStatics.GetAllActorsOfClass` "/Game/KobWar/Controllers/BP_PlayerController.BP_PlayerController_C"))))

(fn `InitGameState`
  (bind _asbp_game_state (cast `/Game/KobWar/GameModeLogic/BP_GameState` (`GameplayStatics.GetGameState`)))
  (bind _output_get (set `self.BPGameState` _asbp_game_state))
  (`/Game/KobWar/GameModeLogic/BP_GameState.UpdateGameData` _output_get (`self.MaxAmountPlayers`) (`self.MaxSpectators`) (`self.AllowClassSelection`) (`self.PlayableClasses`) (`self.IsTeamBased`) (`self.MaxAmountPlayersPerTeam`) (`self.TeamRatio`) (`self.AllowTeamSelection`) (`self.AllowTeamSwitching`) (`self.AllowInbalancedTeamSwitching`) (`self.OtherTeamPlayableClasses`) (`self.SwitchSidesEachRound`) (`self.PreGameWaitTime`)))

(fn `PlayerConnect`
  (params (NewPlayer :type "PlayerController Object Reference"))
  (bind _asbp_player_controller (cast `/Game/KobWar/Controllers/BP_PlayerController` NewPlayer))
  (bind _asbp_player_state (cast `/Game/KobWar/GameModeLogic/BP_PlayerState` (`Controller.PlayerState` NewPlayer)))
  (set `/Game/KobWar/GameModeLogic/BP_PlayerState.PlayerName` (`/Game/KobWar/Controllers/BP_PlayerController.PlayerName` _asbp_player_controller) _asbp_player_state))

(fn `PlayerDisconnect`
  (params (QuitPlayer :type "Controller Object Reference")))

(fn `PlayerSwitchTeam`
  (params (Player :type "PlayerController Object Reference") (TeamId :type Byte))
  (bind _asbp_player_state (cast `/Game/KobWar/GameModeLogic/BP_PlayerState` (`Controller.PlayerState` Player)))
  (set `/Game/KobWar/GameModeLogic/BP_PlayerState.PlayerTeam` TeamId _asbp_player_state))

(fn `RespawnQueuedPlayers`
  (for _array_element (`self.RespawnQueue`)
    (bind _asbp_player_controller (cast `/Game/KobWar/Controllers/BP_PlayerController` _array_element))
    (`/Game/KobWar/Controllers/BP_PlayerController.OwnerTriggerSpawn` _asbp_player_controller)))

(fn `SetPlayerTeam`
  (params (Player :type "PlayerController Object Reference") (Team :type Byte) (ForceSwitch :type Boolean))
  (returns (ReturnValue :type Boolean))
  (locals (Success :type Boolean))
  (bind _bpgamestate (`self.BPGameState`))
  (bind _allowinbalancedteamswitching (`/Game/KobWar/GameModeLogic/BP_GameState.AllowInbalancedTeamSwitching` _bpgamestate))
  (bind _maxamountplayersperteam (`/Game/KobWar/GameModeLogic/BP_GameState.MaxAmountPlayersPerTeam` _bpgamestate))
  (`|ExecutionSequence`
    (:`then_0`
      (`/Engine/EditorBlueprintResources/StandardMacros.IsValid` Player
        (:`Is Valid`
          (bind _asbp_player_state (cast `/Game/KobWar/GameModeLogic/BP_PlayerState` (`Controller.PlayerState` Player)))
          (if (== Team (`/Game/KobWar/GameModeLogic/BP_PlayerState.PlayerTeam` _asbp_player_state))
            (set `local.Success` true)
            (else
              (`/Engine/EditorBlueprintResources/StandardMacros.IsValid` _bpgamestate
                (:`Is Valid`
                  (bind (_spectators _neutralplayers _team1players _team2players) (`/Game/KobWar/GameModeLogic/BP_GameState.GetPlayerCounts` _bpgamestate))
                  (if (== Team (enumliteral `ETeam` "Team_1"))
                    (if (<= _team1players _maxamountplayersperteam)
                      (bind _returnvalue (`KismetMathLibrary.Conv_ByteToDouble` _team1players))
                      (if (== _returnvalue 0.0)
                        (set `local.Success` true)
                        (elif _allowinbalancedteamswitching
                          (set `local.Success` true)
                          (else
                            (bind _returnvalue_2 (`KismetMathLibrary.Conv_ByteToDouble` _team2players))
                            (bind _returnvalue_3 (+ _returnvalue _returnvalue_2))
                            (set `local.Success` (<= (/ _returnvalue _returnvalue_3) (`self.TeamRatio`))))))
                      (else
                        (set `local.Success` false)))
                    (elif (== Team (enumliteral `ETeam` "Team_2"))
                      (if (<= _team2players _maxamountplayersperteam)
                        (if (== _returnvalue_2 0.0)
                          (set `local.Success` true)
                          (elif _allowinbalancedteamswitching
                            (set `local.Success` true)
                            (else
                              (set `local.Success` (<= (/ _returnvalue_2 _returnvalue_3) (- 1.0 (`self.TeamRatio`)))))))
                        (else
                          (set `local.Success` false)))
                      (else
                        (set `local.Success` true)))))))))))
    (:`then_1`
      (if (`local.Success`)
        (`self.PlayerSwitchTeam` Player Team)))
    (:`then_2`
      (return (`local.Success`)))))

(fn `UserConstructionScript`)