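; Preview pawn that shows the player's kobold as the class, team and equipment hovered in class selection.
; On possession it reads appearance and hover state from the player controller.
; It adds eye, horn and gear meshes that follow the body via master pose, colored through dynamic materials.
; Hand equipment is spawned as actors on hand sockets and destroyed with the pawn.
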(event `self.ReceiveBeginPlay`)

(event `self.ReceiveEndPlay`
  (params (EndPlayReason :type "EEndPlayReason Enum" :default "Destroyed"))
  (bind _mainhandequipment (`self.MainhandEquipment`))
  (bind _offhandequipment (`self.OffhandEquipment`))
  (switch `EEndPlayReason` EndPlayReason
    (:`Destroyed`
      (`|ExecutionSequence`
        (:`then_0`
          (`/Engine/EditorBlueprintResources/StandardMacros.IsValid` _mainhandequipment
            (:`Is Valid`
              (`self.K2_DestroyActor` _mainhandequipment))))
        (:`then_1`
          (`/Engine/EditorBlueprintResources/StandardMacros.IsValid` _offhandequipment
            (:`Is Valid`
              (`self.K2_DestroyActor` _offhandequipment))))))))

(event `self.ReceivePossessed`
  (params (NewController :type "Controller Object Reference"))
  (`self.OwnerPossessed`))

(event `OwnerPossessed`
  (`self.InitBodyMat`)
  (`self.InitPlayerCustomizationData`))

(fn `InitBodyMat`
  (bind _bodymesh (`self.BodyMesh`))
  (bind _returnvalue (`PrimitiveComponent.CreateDynamicMaterialInstance` _bodymesh 0 (`PrimitiveComponent.GetMaterial` _bodymesh 0) "None"))
  (`PrimitiveComponent.SetMaterial` _bodymesh 0 _returnvalue)
  (set `self.BodyDynMat` _returnvalue))

(fn `InitPlayerCustomizationData`
  (bind _asbp_player_controller (cast `/Game/KobWar/Controllers/BP_PlayerController` (`GameplayStatics.GetPlayerController` 0)))
  (bind _output_get (set `self.AppearanceData` (`/Game/KobWar/Controllers/BP_PlayerController.AppearanceData` _asbp_player_controller)))
  (`self.LoadAppearanceData` _output_get)
  (bind _bpc_teamclasscontrol (`/Game/KobWar/Controllers/BP_PlayerController.BPC_TeamClassControl` _asbp_player_controller))
  (bind (_charclassname _skeleton) (break `PlayableClassStruct` (`/Game/KobWar/LogicComponents/ControllerTeamClassControl/BPC_TeamClassControl.ClassDataHovered` _bpc_teamclasscontrol)))
  (bind _hoveredequipment (`/Game/KobWar/LogicComponents/ControllerTeamClassControl/BPC_TeamClassControl.HoveredEquipment` _bpc_teamclasscontrol))
  (bind (_gearmesh _bodyoverlaytex _gearmatinst) (`/Game/KobWar/LogicComponents/Appearance/BPFL_GetAppearanceData.LoadCosmetics` _charclassname _hoveredequipment (`/Game/KobWar/LogicComponents/ControllerTeamClassControl/BPC_TeamClassControl.TeamSelected` _bpc_teamclasscontrol)))
  (`self.LoadClassGear` _gearmesh _bodyoverlaytex _gearmatinst)
  (bind (_lightattackdata _heavyattackdata _dodgedata _staggerdata _stagger2data _landdata _weaponskilldata _runningattackdata _backstepdata _specialaction1 _specialaction2 _mainhandclass _offhandclass _animationindex) (`/Game/KobWar/Equipment/BPFL_LoadEquipAnimData.LoadEquipDataByName` 0 0 0 0 _hoveredequipment _skeleton))
  (set `self.AnimIndex` _animationindex)
  (`|ExecutionSequence`
    (:`then_0`
      (bind (_equipclass _color1 _color2 _color3 _matinst) (break `/Game/KobWar/LogicComponents/Equipment/Struct_EquipmentItemData` _mainhandclass))
      (`self.LoadEquipment` (make `/Game/KobWar/LogicComponents/Equipment/Struct_EquipmentItemData` _equipclass _color1 _color2 _color3 _matinst) true))
    (:`then_1`
      (bind (_equipclass_2 _color1_2 _color2_2 _color3_2 _matinst_2) (break `/Game/KobWar/LogicComponents/Equipment/Struct_EquipmentItemData` _offhandclass))
      (`self.LoadEquipment` (make `/Game/KobWar/LogicComponents/Equipment/Struct_EquipmentItemData` _equipclass_2 _color1_2 _color2_2 _color3_2 _matinst_2) false true))))

(fn `LoadAppearanceData`
  (params (Data :type "/Game/KobWar/LogicComponents/Appearance/Struct_AppearanceData Structure"))
  (bind _dynmathorns (`self.DynMatHorns`))
  (bind _eyedynmat (`self.EyeDynMat`))
  (set `self.AppearanceData` Data)
  (`|ExecutionSequence`
    (:`then_0`
      (bind (_eyematinst _valid) (`/Game/KobWar/LogicComponents/Appearance/BPFL_AppearanceData.GetEyesByIndex` (`.Option_Eye_3_DD6C43EE4DFBA57192116C9EA3362334` (break `/Game/KobWar/LogicComponents/Appearance/Struct_AppearanceData` (`self.AppearanceData`)))))
      (if _valid
        (bind _returnvalue (`AddComponent|NODE_AddSkeletalMeshComponent-0`))
        (`SceneComponent.K2_AttachToComponent` _returnvalue (`self.BodyMesh`) "None" "KeepRelative" "KeepRelative" "KeepRelative" true)
        (`SkinnedMeshComponent.SetSkinnedAssetAndUpdate` _returnvalue "/Game/KobWar/CharacterAssets/Kobold/Eyes/kobold_eyes_model.kobold_eyes_model" true)
        (bind _output_get (set `self.SkeletalMeshEyes` _returnvalue))
        (`PrimitiveComponent.SetCollisionResponseToAllChannels` _output_get "ECR_Ignore")
        (`SkinnedMeshComponent.SetLeaderPoseComponent` _returnvalue (`self.BodyMesh`) false)
        (bind _returnvalue_2 (`PrimitiveComponent.CreateDynamicMaterialInstance` _output_get 0 _eyematinst "None"))
        (bind _output_get_2 (set `self.EyeDynMat` _returnvalue_2))
        (`PrimitiveComponent.SetMaterial` _returnvalue 0 _output_get_2)
        (bind (_color1 _color2 _color3) (`/Game/KobWar/LogicComponents/Appearance/BPFL_AppearanceData.GetEyesColors` (`.Option_EyeColor_5_497B70AD40D62BFC9B08D2A2F0AB5A7B` (break `/Game/KobWar/LogicComponents/Appearance/Struct_AppearanceData` (`self.AppearanceData`)))))
        (`MaterialInstanceDynamic.SetVectorParameterValue` _eyedynmat "Color1" _color1)
        (`MaterialInstanceDynamic.SetVectorParameterValue` _eyedynmat "Color2" _color2)
        (`MaterialInstanceDynamic.SetVectorParameterValue` _eyedynmat "Color3" _color3)))
    (:`then_1`
      (bind (_hornmesh _valid_2) (`/Game/KobWar/LogicComponents/Appearance/BPFL_AppearanceData.GetHornsByIndex` (`.Option_Horn_7_5C7E533B4619FE7C435941AB51A0F3BC` (break `/Game/KobWar/LogicComponents/Appearance/Struct_AppearanceData` (`self.AppearanceData`)))))
      (if _valid_2
        (bind _returnvalue_3 (`AddComponent|NODE_AddSkeletalMeshComponent-1`))
        (`SceneComponent.K2_AttachToComponent` _returnvalue_3 (`self.BodyMesh`) "None" "KeepRelative" "KeepRelative" "KeepRelative" true)
        (`SkinnedMeshComponent.SetSkinnedAssetAndUpdate` _returnvalue_3 _hornmesh true)
        (bind _output_get_3 (set `self.SkeletalMeshHorns` _returnvalue_3))
        (`PrimitiveComponent.SetCollisionResponseToAllChannels` _output_get_3 "ECR_Ignore")
        (`SkinnedMeshComponent.SetLeaderPoseComponent` _output_get_3 (`self.BodyMesh`) false)
        (bind _returnvalue_4 (`PrimitiveComponent.CreateDynamicMaterialInstance` _output_get_3 0 (`PrimitiveComponent.GetMaterial` _output_get_3 0) "None"))
        (set `self.DynMatHorns` _returnvalue_4)
        (`PrimitiveComponent.SetMaterial` _output_get_3 0 _returnvalue_4)
        (bind (_color1_2 _color2_2 _color3_2) (`/Game/KobWar/LogicComponents/Appearance/BPFL_AppearanceData.GetHornsColor` (`.Option_HornColor_9_BE6E49C54AB9768E2FE5C9A4B833C3A6` (break `/Game/KobWar/LogicComponents/Appearance/Struct_AppearanceData` (`self.AppearanceData`)))))
        (`MaterialInstanceDynamic.SetVectorParameterValue` _dynmathorns "Color1" _color1_2)
        (`MaterialInstanceDynamic.SetVectorParameterValue` _dynmathorns "Color2" _color2_2)
        (`MaterialInstanceDynamic.SetVectorParameterValue` _dynmathorns "Color3" _color3_2)))))

(fn `LoadClassGear`
  (params (GearMesh :type "SkeletalMesh Object Reference") (BodyOverlayTex :type "Texture Object Reference") (GearMatInst :type "MaterialInstance Object Reference"))
  (bind _skeletalgearmesh (`self.SkeletalGearMesh`))
  (bind _bodymesh (`self.BodyMesh`))
  (bind _skeletalgearmesh_2 (`self.SkeletalGearMesh`))
  (bind _bodydynmat (`self.BodyDynMat`))
  (`|ExecutionSequence`
    (:`then_0`
      (`/Engine/EditorBlueprintResources/StandardMacros.IsValid` _skeletalgearmesh
        (:`Is Valid`
          (`ActorComponent.K2_DestroyComponent` _skeletalgearmesh)
          (set `self.SkeletalGearMesh` null))
        (:`Is Not Valid`
          _))
      (`/Engine/EditorBlueprintResources/StandardMacros.IsValid` GearMesh
        (:`Is Valid`
          (bind _returnvalue (`AddComponent|NODE_AddSkeletalMeshComponent-2`))
          (bind _output_get (set `self.SkeletalGearMesh` _returnvalue))
          (`PrimitiveComponent.SetCollisionEnabled` _returnvalue "NoCollision")
          (`PrimitiveComponent.SetCollisionEnabled` _output_get "NoCollision")
          (`SceneComponent.K2_AttachToComponent` _output_get _bodymesh "None" "KeepRelative" "KeepRelative" "KeepRelative" true)
          (`SkinnedMeshComponent.SetSkinnedAssetAndUpdate` _returnvalue GearMesh true)
          (`SkinnedMeshComponent.SetSkinnedAssetAndUpdate` _output_get GearMesh true)
          (`SkinnedMeshComponent.SetLeaderPoseComponent` _skeletalgearmesh _bodymesh false)
          (`SkinnedMeshComponent.SetLeaderPoseComponent` _returnvalue _bodymesh false)
          (`SkinnedMeshComponent.SetLeaderPoseComponent` _output_get _bodymesh false))))
    (:`then_1`
      (`/Engine/EditorBlueprintResources/StandardMacros.IsValid` _skeletalgearmesh_2
        (:`Is Valid`
          (`/Engine/EditorBlueprintResources/StandardMacros.IsValid` GearMatInst
            (:`Is Valid`
              (bind _returnvalue_2 (`KismetMaterialLibrary.CreateDynamicMaterialInstance` GearMatInst))
              (`PrimitiveComponent.SetMaterial` _skeletalgearmesh_2 0 _returnvalue_2)
              (bind _output_get_2 (set `self.GearDynMat` _returnvalue_2))
              (`MaterialInstanceDynamic.SetVectorParameterValue` _output_get_2 "Color1" (struct :`R` 1.0 :`G` 1.0 :`B` 1.0 :`A` 1.0))
              (`MaterialInstanceDynamic.SetVectorParameterValue` _output_get_2 "Color2" (struct :`R` 1.0 :`G` 1.0 :`B` 1.0 :`A` 1.0))
              (`MaterialInstanceDynamic.SetVectorParameterValue` _output_get_2 "Color3" (struct :`R` 1.0 :`G` 1.0 :`B` 1.0 :`A` 1.0)))))))
    (:`then_2`
      (`/Engine/EditorBlueprintResources/StandardMacros.IsValid` _bodydynmat
        (:`Is Valid`
          (`/Engine/EditorBlueprintResources/StandardMacros.IsValid` BodyOverlayTex
            (:`Is Valid`
              (`MaterialInstanceDynamic.SetTextureParameterValue` _bodydynmat "ColorTex3Param" BodyOverlayTex))))))))

(fn `LoadEquipment`
  (params (Equipment :type "/Game/KobWar/LogicComponents/Equipment/Struct_EquipmentItemData Structure") (Mainhand :type Boolean) (Offhand :type Boolean))
  (bind _mainhandequipment (`self.MainhandEquipment`))
  (bind _offhandequipment (`self.OffhandEquipment`))
  (`|ExecutionSequence`
    (:`then_0`
      (if Mainhand
        (`/Engine/EditorBlueprintResources/StandardMacros.IsValid` _mainhandequipment
          (:`Is Valid`
            (`self.K2_DestroyActor` _mainhandequipment)
            (set `self.MainhandDynMat` null)))))
    (:`then_1`
      (if Offhand
        (`/Engine/EditorBlueprintResources/StandardMacros.IsValid` _offhandequipment
          (:`Is Valid`
            (`self.K2_DestroyActor` _offhandequipment)
            (set `self.OffhandDynMat` null)))))
    (:`then_2`
      (if (`KismetSystemLibrary.IsValidClass` Equipment_EquipClass_2_E196BC70449D8ED7FDEDF695EE5B3600)
        (if (or Mainhand Offhand)
          (bind _returnvalue (`|SpawnActorFromClass` Equipment_EquipClass_2_E196BC70449D8ED7FDEDF695EE5B3600 (`KismetMathLibrary.MakeTransform` (0.0 0.0 0.0)) "AlwaysSpawn" "OverrideRootScale" self self))
          (if Mainhand
            (`self.K2_AttachToComponent` _returnvalue (`self.BodyMesh`) "item_R" "KeepRelative" "KeepRelative" "KeepWorld" true)
            (bind _output_get (set `self.MainhandEquipment` _returnvalue))
            (bind _staticmesh (`/Game/KobWar/Equipment/BP_HeldEquipment.StaticMesh` _output_get))
            (bind _returnvalue_2 (`PrimitiveComponent.CreateDynamicMaterialInstance` _staticmesh 0 Equipment_MatInst_19_80E6ECEA489706C743323586ACFB71D1 "None"))
            (bind _output_get_2 (set `self.MainhandDynMat` _returnvalue_2))
            (`PrimitiveComponent.SetMaterial` _staticmesh 0 _output_get_2)
            (`MaterialInstanceDynamic.SetVectorParameterValue` :`self` _output_get_2 :`ParameterName` "Color1")
            (`MaterialInstanceDynamic.SetVectorParameterValue` :`self` _output_get_2 :`ParameterName` "Color2")
            (`MaterialInstanceDynamic.SetVectorParameterValue` :`self` _output_get_2 :`ParameterName` "Color3")
            (elif Offhand
              (`self.K2_AttachToComponent` _returnvalue (`self.BodyMesh`) "item_L" "KeepRelative" "KeepRelative" "KeepWorld" true)
              (bind _output_get_3 (set `self.OffhandEquipment` _returnvalue))
              (bind _staticmesh_2 (`/Game/KobWar/Equipment/BP_HeldEquipment.StaticMesh` _output_get_3))
              (bind _returnvalue_3 (`PrimitiveComponent.CreateDynamicMaterialInstance` _staticmesh_2 0 Equipment_MatInst_19_80E6ECEA489706C743323586ACFB71D1 "None"))
              (bind _output_get_4 (set `self.OffhandDynMat` _returnvalue_3))
              (`PrimitiveComponent.SetMaterial` _staticmesh_2 0 _output_get_4)
              (`MaterialInstanceDynamic.SetVectorParameterValue` :`self` _output_get_4 :`ParameterName` "Color1")
              (`MaterialInstanceDynamic.SetVectorParameterValue` :`self` _output_get_4 :`ParameterName` "Color2")
              (`MaterialInstanceDynamic.SetVectorParameterValue` :`self` _output_get_4 :`ParameterName` "Color3"))))))))

(fn `UserConstructionScript`)