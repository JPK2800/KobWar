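; BP_GameState is the game state for KobWar that stores the match's rule configuration.
; A single UpdateGameData event in the ServerData graph copies its inputs into member variables, with no validation or other logic.
; The stored settings cover player and spectator limits, class selection, team balance and switching, per-round side swaps and pre-game wait time.
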(event `UpdateGameData`
  (params (MaxAmountPlayers :type Byte) (MaxSpectators :type Byte) (AllowClassSelection :type Boolean) (PlayableClasses :type "Array of PlayableClassStruct Structure") (IsTeamBased :type Boolean) (MaxAmountPlayersPerTeam :type Byte) (TeamRatio :type "Float (double-precision)") (AllowTeamSelection :type Boolean) (AllowTeamSwitching :type Boolean) (AllowInbalancedTeamSwitching :type Boolean) (OtherTeamPlayableClasses :type "Array of PlayableClassStruct Structure") (SwitchSideEachRound :type Boolean) (PreGameWaitTime :type "Float (double-precision)"))
  (set `self.MaxAmountPlayers` MaxAmountPlayers)
  (set `self.MaxSpectators` MaxSpectators)
  (set `self.AllowClassSelection` AllowClassSelection)
  (set `self.PlayableClasses` PlayableClasses)
  (set `self.IsTeamBased` IsTeamBased)
  (set `self.MaxAmountPlayersPerTeam` MaxAmountPlayersPerTeam)
  (set `self.TeamRatio` TeamRatio)
  (set `self.AllowTeamSelection` AllowTeamSelection)
  (set `self.AllowTeamSwitching` AllowTeamSwitching)
  (set `self.AllowInbalancedTeamSwitching` AllowInbalancedTeamSwitching)
  (set `self.OtherTeamPlayableClasses` OtherTeamPlayableClasses)
  (set `self.SwitchSideEachRound` SwitchSideEachRound)
  (set `self.PreGameWaitTime` PreGameWaitTime))

(fn `UserConstructionScript`)