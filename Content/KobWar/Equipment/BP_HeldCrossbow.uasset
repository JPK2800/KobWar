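; Held crossbow equipment that switches between loaded and unloaded meshes and drives a projectile control component with its ready and aiming states.
; Trigger events load or unload it; BeginPlay starts it loaded.
; The locally controlled owner applies loaded changes immediately and forwards them to the server, with IsLoaded using a RepNotify.
; When the component signals a new spline, the crossbow rebuilds thin spline mesh components along it using the projectile material.
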(event `self.ReceiveBeginPlay`
  (`parent.ReceiveBeginPlay`)
  (`self.LocalUpdateLoaded` true)
  (`/Game/KobWar/Equipment/BPC_ProjectileControlComp.InitSplineComponent` (`self.BPC_ProjectileControlComp`) (`self.Spline`)))

(event `self.BPC_ProjectileControlComp.OnNewSpline`
  (bind _spline (`self.Spline`))
  (bind _splinemeshcomps (`self.SplineMeshComps`))
  (`|ExecutionSequence`
    (:`then_0`
      (for _array_element _splinemeshcomps
        (`ActorComponent.K2_DestroyComponent` _array_element)))
    (:`then_1`
      (`KismetArrayLibrary.Array_Clear` _splinemeshcomps)
      (for _index (range (+ (- (`SplineComponent.GetNumberOfSplinePoints` _spline) 2) 1))
        (bind (_returnvalue_location _returnvalue_rotation) (`KismetMathLibrary.BreakTransform` (`SplineComponent.GetTransformAtSplinePoint` _spline _index "Local" false)))
        (bind _returnvalue (`AddComponent|NODE_AddSplineMeshComponent-1` :`bManualAttachment` true :`RelativeTransform` (`KismetMathLibrary.MakeTransform` _returnvalue_location _returnvalue_rotation (`KismetMathLibrary.MakeVector` 1.334 0.01 0.01))))
        (`KismetArrayLibrary.Array_Add` (`self.SplineMeshComps`) _returnvalue)
        (`PrimitiveComponent.SetMaterial` _returnvalue 0 (`self.ProjectileMaterial`))))))

(event `LocalUpdateLoaded`
  (params (Loaded :type Boolean))
  (bind _aspawn (cast `Pawn` (`self.GetOwner`)))
  (if (`Pawn.IsLocallyControlled` _aspawn)
    (`self.ServerUpdateLoaded` Loaded)
    (`self.UpdateLoaded` Loaded)))

(event `ServerUpdateLoaded`
  (params (Loaded :type Boolean))
  (bind _aspawn (cast `Pawn` (`self.GetOwner`)))
  (if (not (`Pawn.IsLocallyControlled` _aspawn))
    (`self.UpdateLoaded` Loaded)))

(fn `OnRep_IsLoaded`
  (`self.UpdateLoaded` (`self.IsLoaded`)))

(fn `TriggerEvent1`
  (`parent.TriggerEvent1`)
  (`self.LocalUpdateLoaded` true))

(fn `TriggerEvent2`
  (`parent.TriggerEvent2`)
  (`self.LocalUpdateLoaded` false))

(fn `UpdateIsAiming`
  (params (Toggle :type Boolean))
  (`parent.UpdateIsAiming` Toggle)
  (`/Game/KobWar/Equipment/BPC_ProjectileControlComp.UpdateAiming` (`self.BPC_ProjectileControlComp`) Toggle))

(fn `UpdateLoaded`
  (params (Loaded :type Boolean))
  (if (!= Loaded (`self.IsLoaded`))
    (bind _output_get (set `self.IsLoaded` Loaded))
    (`SceneComponent.SetVisibility` (`self.StaticMesh`) _output_get false)
    (`SceneComponent.SetVisibility` (`self.UnloadedCrossbow`) (not _output_get) false)
    (`/Game/KobWar/Equipment/BPC_ProjectileControlComp.UpdateReady` (`self.BPC_ProjectileControlComp`) _output_get)))

(fn `UserConstructionScript`
  (`parent.UserConstructionScript`))