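; Component for held equipment that previews a projectile's arc while the owning player aims.
; When ready and locally controlled, each tick predicts the path from control rotation, velocity and custom gravity against WorldStatic objects.
; The path rebuilds a supplied spline as linear points and fires OnNewSpline to notify listeners.
; UpdateAiming toggles ticking; leaving aim or ready state clears the preview.
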(event `self.ReceiveBeginPlay`
  (`self.InitOwner`))

(event `self.ReceiveTick`
  (params (DeltaSeconds :type "Float (single-precision)"))
  (`self.PredictAimStep` DeltaSeconds))

(fn `ClearAimPreview`
  (`SplineComponent.ClearSplinePoints` (`self.AimSpline`) true)
  (`self.OnNewSpline`))

(fn `InitOwner`
  (bind _asbp_held_equipment (cast `/Game/KobWar/Equipment/BP_HeldEquipment` (`self.GetOwner`)))
  (`/Engine/EditorBlueprintResources/StandardMacros.IsValid` _asbp_held_equipment
    (:`Is Valid`
      (bind _output_get (set `self.Equipment` _asbp_held_equipment))
      (bind _asbp_player_character_base (cast `/Game/KobWar/BP_PlayerCharacterBase` (`Actor.GetOwner` _output_get)))
      (`/Engine/EditorBlueprintResources/StandardMacros.IsValid` _asbp_player_character_base
        (:`Is Valid`
          (set `self.OwnerChar` _asbp_player_character_base))))))

(fn `InitSplineComponent`
  (params (SplineComp :type "SplineComponent Object Reference"))
  (set `self.AimSpline` SplineComp))

(fn `PredictAimStep`
  (params (DeltaTime :type "Float (double-precision)"))
  (bind _aimspline (`self.AimSpline`))
  (bind _ownerchar (`self.OwnerChar`))
  (bind _returnvalue (`Pawn.GetControlRotation` _ownerchar))
  (`/Engine/EditorBlueprintResources/StandardMacros.IsValid` _ownerchar
    (:`Is Valid`
      (if (`Pawn.IsLocallyControlled` _ownerchar)
        (if (`self.IsReady`)
          (bind (_outhit _outpathpositions) (`GameplayStatics.Blueprint_PredictProjectilePath_ByObjectType` (+ (`Actor.K2_GetActorLocation` _ownerchar) (`KismetMathLibrary.GreaterGreater_VectorRotator` (`self.ProjectileSpawnOffset`) _returnvalue)) (* (`KismetMathLibrary.GetForwardVector` _returnvalue) (`self.ProjectileVelocity`)) true (`self.ProjectileRadius`) (`|MakeArray` "ObjectTypeQuery1" :!type "EObjectTypeQuery Enum") false (`|MakeArray` (`self.GetOwner`)) "None" 0.0 15.0 2.5 (`self.ProjectileGravityZ`)))
          (`SplineComponent.ClearSplinePoints` _aimspline true)
          (for (_array_element _array_index) _outpathpositions
            (`SplineComponent.AddSplinePoint` _aimspline _array_element "Local" true)
            (`SplineComponent.SetSplinePointType` _aimspline _array_index "Linear" true))
          (`self.OnNewSpline`))))))

(fn `UpdateAiming`
  (params (Toggle :type Boolean))
  (bind _output_get (set `self.IsAiming` Toggle))
  (`self.SetComponentTickEnabled` _output_get)
  (`|ExecutionSequence`
    (:`then_0`
      (if (not _output_get)
        (`self.ClearAimPreview`)))
    (:`then_1`
      (`/Engine/EditorBlueprintResources/StandardMacros.IsValid` (`self.AimSpline`)
        (:`Is Not Valid`
          (`KismetSystemLibrary.PrintString` "Spline is null in BPC_ProjectileControlComp"))))))

(fn `UpdateReady`
  (params (Toggle :type Boolean))
  (bind _output_get (set `self.IsReady` Toggle))
  (if _output_get
    (`self.UpdateAiming` true)
    (else
      (`self.ClearAimPreview`))))