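; Hitzone component for held equipment that detects hits on player characters while line hits are enabled.
; Each tick it line-traces between adjacent child components and back to their previous positions, covering the swept area.
; The owning client toggles tracing locally and on the server, with an OnRep mirroring the state.
; Each character is hit once per activation, filtered by team, and receives fixed damage through its hit receiver component.
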(event `self.ReceiveBeginPlay`
  (`self.LoadChildComponents`)
  (`self.InitOwner`))

(event `self.ReceiveTick`
  (params (DeltaSeconds :type "Float (single-precision)"))
  (`self.LineHitStep` DeltaSeconds))

(event `LocalToggleHits`
  (params (Toggle :type Boolean))
  (if (`Pawn.IsLocallyControlled` (`self.Owner`))
    (`self.ServerToggleHits` Toggle)
    (`self.ToggleLineHits` Toggle)
    (set `self.IsLineHitEnabled` Toggle)))

(event `ServerToggleHits`
  (params (Toggle :type Boolean))
  (bind _output_get (set `self.IsLineHitEnabled` Toggle))
  (`self.ToggleLineHits` _output_get))

(fn `HitCharacter`
  (params (Character :type "/Game/KobWar/BP_PlayerCharacterBase Object Reference"))
  (bind _returnvalue (enumliteral `ETeam` "NeutralTeam"))
  (bind _owner (`self.Owner`))
  (bind _genericteamid (`KobWarCharacter.GenericTeamId` Character))
  (bind _bpc_hitreceivercomponent (`/Game/KobWar/BP_PlayerCharacterBase.BPC_HitReceiverComponent` Character))
  (`/Engine/EditorBlueprintResources/StandardMacros.IsValid` _owner
    (:`Is Valid`
      (if (!= Character _owner)
        (bind _returnvalue_2 (`KobWarCharacter.GetCharacterTeamId` _owner))
        (if (or (!= _returnvalue_2 _genericteamid) (== _returnvalue_2 _returnvalue) (== _genericteamid _returnvalue))
          (`KismetSystemLibrary.PrintString` (`KismetStringLibrary.Concat_StrStr` "Hit target " (`KismetSystemLibrary.GetDisplayName` Character)))
          (`/Engine/EditorBlueprintResources/StandardMacros.IsValid` _bpc_hitreceivercomponent
            (:`Is Valid`
              (`/Game/KobWar/LogicComponents/HitReceiverComponent/BPC_HitReceiverComponent.LocalTakeHit` _bpc_hitreceivercomponent (make `/Game/KobWar/LogicComponents/HitReceiverComponent/Struct_TakeHitData` (`self.Owner`) false false false false 5 (`|MakeArray`))))))))))

(fn `InitOwner`
  (bind _asbp_held_equipment (cast `/Game/KobWar/Equipment/BP_HeldEquipment` (`self.GetOwner`)))
  (bind _output_get (set `self.EquipmentOwner` _asbp_held_equipment))
  (bind _asbp_player_character_base (cast `/Game/KobWar/BP_PlayerCharacterBase` (`Actor.GetOwner` _output_get)))
  (set `self.Owner` _asbp_player_character_base))

(fn `LineHitStep`
  (params (DeltaTime :type "Float (double-precision)"))
  (locals (NewPrevPositions :type "Array of Vector Structure"))
  (bind _array (`|MakeArray` "ObjectTypeQuery3" :!type "EObjectTypeQuery Enum"))
  (bind _childcomponents (`self.ChildComponents`))
  (bind _prevpositions (`self.PrevPositions`))
  (bind _array_2 (`|MakeArray` (`self.GetOwner`)))
  (if (`self.IsLineHitEnabled`)
    (for (_array_element _array_index) _childcomponents
      (bind _returnvalue (`self.K2_GetComponentLocation` _array_element))
      (`KismetArrayLibrary.Array_Add` (`local.NewPrevPositions`) _returnvalue)
      (`|ExecutionSequence`
        (:`then_0`
          (if (!= _array_index 0)
            (bind _outhit (`KismetSystemLibrary.LineTraceSingleForObjects` _returnvalue (`self.K2_GetComponentLocation` (`|GetArrayItem` _childcomponents (- _array_index 1))) _array false _array_2 "ForOneFrame"))
            (bind _asbp_player_character_base (cast `/Game/KobWar/BP_PlayerCharacterBase` (`.HitActor` (`GameplayStatics.BreakHitResult` _outhit))))
            (if (not (`KismetArrayLibrary.Array_Contains` (`self.HitActors`) _asbp_player_character_base))
              (`KismetArrayLibrary.Array_Add` (`self.HitActors`) _asbp_player_character_base)
              (`self.HitCharacter` _asbp_player_character_base))))
        (:`then_1`
          (if (`KismetArrayLibrary.Array_IsValidIndex` _prevpositions _array_index)
            (bind _outhit_2 (`KismetSystemLibrary.LineTraceSingleForObjects` _returnvalue (`|GetArrayItem` _prevpositions _array_index) _array false _array_2 "ForOneFrame"))
            (bind _asbp_player_character_base_2 (cast `/Game/KobWar/BP_PlayerCharacterBase` (`.HitActor` (`GameplayStatics.BreakHitResult` _outhit_2))))
            (if (not (`KismetArrayLibrary.Array_Contains` (`self.HitActors`) _asbp_player_character_base_2))
              (`KismetArrayLibrary.Array_Add` (`self.HitActors`) _asbp_player_character_base_2)
              (`self.HitCharacter` _asbp_player_character_base_2))))))
    (set `self.PrevPositions` (`local.NewPrevPositions`))))

(fn `LoadChildComponents`
  (set `self.ChildComponents` (`self.GetChildrenComponents` true)))

(fn `OnRep_IsLineHitEnabled`
  (`self.ToggleLineHits` (`self.IsLineHitEnabled`)))

(fn `ToggleLineHits`
  (params (Toggle :type Boolean))
  (`KismetArrayLibrary.Array_Clear` (`self.HitActors`))
  (`KismetArrayLibrary.Array_Clear` (`self.PrevPositions`))
  (`self.SetComponentTickEnabled` Toggle))