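; Crossbow bolt projectile that sticks into whatever it hits.
; A hitzone component's TargetHit attaches the bolt to the receiver's mesh, while StopCollision overlaps attach it only to StaticMeshActors, both keeping world transform.
; Either hit then freezes the bolt by zeroing projectile gravity and velocity, deactivating the hitzone and disabling StopCollision.
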(event `self.ReceiveBeginPlay`
  (`parent.ReceiveBeginPlay`))

(event `self.BPC_EquipHitzone.TargetHit`
  (params (Data :type "/Game/KobWar/LogicComponents/HitReceiverComponent/Struct_TakeHitData Structure") (HitReceiver :type "/Game/KobWar/BP_PlayerCharacterBase Object Reference"))
  (`self.HitAttachToPlayer` HitReceiver))

(event `self.StopCollision.OnComponentBeginOverlap`
  (params (OverlappedComponent :type "PrimitiveComponent Object Reference") (OtherActor :type "Actor Object Reference") (OtherComp :type "PrimitiveComponent Object Reference") (OtherBodyIndex :type Integer) (bFromSweep :type Boolean) (SweepResult :type "HitResult Structure (by ref)"))
  (`self.HitAttachToMesh` OtherActor))

(fn `DeactivateMovement`
  (bind _projectilemovement (`self.ProjectileMovement`))
  (bind _bpc_equiphitzone (`self.BPC_EquipHitzone`))
  (bind _stopcollision (`self.StopCollision`))
  (set `ProjectileMovementComponent.ProjectileGravityScale` 0.0 _projectilemovement)
  (set `MovementComponent.Velocity` (0.0 0.0 0.0) _projectilemovement)
  (`ActorComponent.SetComponentTickEnabled` _bpc_equiphitzone false)
  (`ActorComponent.Deactivate` _bpc_equiphitzone)
  (`PrimitiveComponent.SetCollisionEnabled` _stopcollision "NoCollision")
  (set `PrimitiveComponent.bGenerateOverlapEvents` false _stopcollision))

(fn `HitAttachToMesh`
  (params (Target :type "Actor Object Reference"))
  (if (!= Target self)
    (bind _asstatic_mesh_actor (cast `StaticMeshActor` Target))
    (`self.K2_AttachToActor` _asstatic_mesh_actor "None" "KeepWorld" "KeepWorld" "KeepWorld")
    (`self.DeactivateMovement`)))

(fn `HitAttachToPlayer`
  (params (Target :type "/Game/KobWar/BP_PlayerCharacterBase Object Reference"))
  (bind _mesh (`Character.Mesh` Target))
  (if (!= Target self)
    (`/Engine/EditorBlueprintResources/StandardMacros.IsValid` Target
      (:`Is Valid`
        (`/Engine/EditorBlueprintResources/StandardMacros.IsValid` _mesh
          (:`Is Valid`
            (`self.K2_AttachToComponent` _mesh "None" "KeepWorld" "KeepWorld" "KeepWorld")
            (`self.DeactivateMovement`)))))))

(fn `UserConstructionScript`
  (`parent.UserConstructionScript`))