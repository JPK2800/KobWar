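; BP_TrajectoryActor is an equipment actor that displays a trajectory as a thin tube of spline meshes with an end marker.
; Every Tick, DrawTrajectoryStep destroys and recreates one SplineMesh component per SplinePath segment, using local-space locations and tangents.
; EndPathStaticMesh moves to the last spline point.
; The spline points are not set in this Blueprint, and the segment meshes are destroyed with the actor.
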(event `self.ReceiveBeginPlay`)

(event `self.ReceiveTick`
  (params (DeltaSeconds :type "Float (single-precision)"))
  (`self.DrawTrajectoryStep` DeltaSeconds))

(event `self.ReceiveDestroyed`
  (for _array_element (`self.SplineMesh`)
    (`ActorComponent.K2_DestroyComponent` _array_element))
  (`parent.ReceiveDestroyed`))

(fn `DrawTrajectoryStep`
  (params (DeltaTime :type "Float (double-precision)"))
  (bind _splinepath (`self.SplinePath`))
  (bind _endpathstaticmesh (`self.EndPathStaticMesh`))
  (bind _returnvalue (`SplineComponent.GetNumberOfSplinePoints` _splinepath))
  (`/Engine/EditorBlueprintResources/StandardMacros.IsValid` _splinepath
    (:`Is Valid`
      (`|ExecutionSequence`
        (:`then_0`
          (for _array_element (`self.SplineMesh`)
            (`ActorComponent.K2_DestroyComponent` _array_element))
          (`KismetArrayLibrary.Array_Clear` (`self.SplineMesh`))
          (`SceneComponent.SetVisibility` (`self.EndPathStaticMesh`) false false))
        (:`then_1`
          (for _index (range (+ (- _returnvalue 2) 1))
            (bind _returnvalue_2 (`AddComponent|NODE_AddSplineMeshComponent-0`))
            (`SplineMeshComponent.SetStartScale` _returnvalue_2 (0.2 0.2) true)
            (`SplineMeshComponent.SetEndScale` _returnvalue_2 (0.2 0.2) true)
            (bind (_location _tangent) (`SplineComponent.GetLocationAndTangentAtSplinePoint` _splinepath _index "Local"))
            (bind (_location_2 _tangent_2) (`SplineComponent.GetLocationAndTangentAtSplinePoint` _splinepath (+ _index 1) "Local"))
            (`SplineMeshComponent.SetStartAndEnd` _returnvalue_2 _location _tangent _location_2 _tangent_2 true)
            (`KismetArrayLibrary.Array_Add` (`self.SplineMesh`) _returnvalue_2))
          (`SceneComponent.SetVisibility` _endpathstaticmesh true false)
          (`SceneComponent.K2_SetRelativeLocation` _endpathstaticmesh (`SplineComponent.GetLocationAtSplinePoint` _splinepath (- _returnvalue 1) "Local") false true))))))

(fn `UserConstructionScript`)