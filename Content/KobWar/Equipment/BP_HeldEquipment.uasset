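; BP_HeldEquipment is a held equipment actor that manages the hit zones used for its hit detection.
; On BeginPlay it gathers its BPC_EquipHitzone components into the HitboxZones map, keyed by each component's HitboxIndex.
; ToggleSpecificHitzone switches line hits on or off for one index if it exists in the map, and ToggleAllHitzones applies this to every key.
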(event `self.ReceiveBeginPlay`
  (`self.InitHitzones`))

(fn `InitHitzones`
  (for _array_element (`self.K2_GetComponentsByClass` "/Game/KobWar/Equipment/BPC_EquipHitzone.BPC_EquipHitzone_C")
    (`BlueprintMapLibrary.Map_Add` (`self.HitboxZones`) (`/Game/KobWar/Equipment/BPC_EquipHitzone.HitboxIndex` _array_element) _array_element)))

(fn `ToggleAllHitzones`
  (params (Enable :type Boolean))
  (bind _keys (`BlueprintMapLibrary.Map_Keys` (`self.HitboxZones`)))
  (for _array_element _keys
    (`self.ToggleSpecificHitzone` _array_element Enable)))

(fn `ToggleSpecificHitzone`
  (params (HitboxIndex :type Byte) (Enable :type Boolean))
  (bind (_value _returnvalue) (`BlueprintMapLibrary.Map_Find` (`self.HitboxZones`) HitboxIndex))
  (if _returnvalue
    (`/Game/KobWar/Equipment/BPC_EquipHitzone.ToggleLineHits` _value Enable)))

(fn `UserConstructionScript`)